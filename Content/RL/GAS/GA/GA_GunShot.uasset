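; GAS ability that fires a gun for either a VR player pawn or a monster, with the weapon as owner actor.
; After commit, it spawns a bullet carrying an effect container from the weapon or monster fire position and plays a muzzle cue.
; It waits for one bullet-hit event, applies the container and impact cue, then ends.
; For the player, it also plays the shoot animation and removes gunshot cooldown during bullet time.
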(event `self.K2_ActivateAbility`
  (bind _returnvalue (`self.GetAbilityLevel`))
  (bind (_owneractor _avataractor) (break `GameplayAbilityActorInfo` (`self.GetActorInfo`)))
  (bind _returnvalue_2 (`self.K2_CommitAbility`))
  (if _returnvalue_2
    (bind _asbp_vr_pawn (cast `/Game/RL/Core/BP_VR_Pawn` _avataractor)
      (:`then`
        (bind _asbp_weapon_base (cast `/Game/RL/Weapon/BP_WeaponBase` _owneractor))
        (`/Game/RL/Weapon/BP_WeaponBase.PlayShootAnimation` _asbp_weapon_base)
        (`/Game/RL/Weapon/BP_WeaponBase.SpawnBullet` :`self` _asbp_weapon_base :`Transform` (`/Game/RL/Weapon/BP_WeaponBase.GetWeaponFirePosition` _asbp_weapon_base) :`Container` (`BlueprintMapLibrary.Map_Find` (`self.EffectContainerMap`) (struct :`TagName` "Event.Shared.WeaponHit.Bullet")) :`Level` (`self.GetAbilityLevel`))
        (`|ExecutionSequence`
          (:`then_0`
            (bind (_returnvalue_location _returnvalue_rotation) (`KismetMathLibrary.BreakTransform` (`/Game/RL/Weapon/BP_WeaponBase.GetMuzzleTransform` _asbp_weapon_base)))
            (`self.K2_AddGameplayCueWithParams` (struct :`TagName` "GameplayCue.BulletMuzzle.Default") (`AbilitySystemBlueprintLibrary.MakeGameplayCueParameters` 0.0 0.0 (struct) (struct) (struct) (struct) (struct) _returnvalue_location (`KismetMathLibrary.Conv_RotatorToVector` _returnvalue_rotation) null _asbp_weapon_base) false)
            (bind (_asynctaskproxy _payload) (`AbilityAsync_WaitGameplayEvent.WaitGameplayEventToActor` (`self.GetAvatarActorFromActorInfo`) (struct :`TagName` "Event.Shared.WeaponHit.Bullet") true :!label _label)
              (:`EventReceived`
                (bind (_eventtag _instigator _target _optionalobject _optionalobject2 _contexthandle _instigatortags _targettags _eventmagnitude _targetdata) (break `GameplayEventData` _payload))
                (bind (_bblockinghit _binitialoverlap _time _distance _location _impactpoint _normal _impactnormal _physmat _hitactor _hitcomponent) (`GameplayStatics.BreakHitResult` (`AbilitySystemBlueprintLibrary.GetHitResultFromTargetData` _targetdata)))
                (`KismetSystemLibrary.PrintString` (`KismetStringLibrary.Concat_StrStr` "子弹打中了= " (`KismetSystemLibrary.GetDisplayName` _hitactor) " \n组件=" (`KismetSystemLibrary.GetDisplayName` _hitcomponent)) false)
                (`self.ApplyEffectContainer` _eventtag _payload)
                (`self.K2_AddGameplayCueWithParams` (`self.Tag_HitCue`) (`AbilitySystemBlueprintLibrary.MakeGameplayCueParameters` 0.0 0.0 _contexthandle (struct) (struct) (struct) (struct) _impactpoint _impactnormal _instigator _instigator _optionalobject2 _physmat _returnvalue _returnvalue) false)
                (`self.K2_EndAbility`))))
          (:`then_1`
            (if (`BlueprintGameplayTagLibrary.HasTag` (`FGComponent.GetAllTags` (`FGCharacter.AbilitySystemComponent` _asbp_vr_pawn)) (struct :`TagName` "State.BulletTime"))
              (`self.BP_RemoveGameplayEffectFromOwnerWithAssetTags` (struct :`GameplayTags` (struct :`(TagName` "Cooldown.GunShoot.Default") :`(TagName` "Cooldown.GunShoot.Pistol.01"))))))))
      (:`CastFailed`
        (bind _asbp_monster_base (cast `/Game/RL/AI/BP_MonsterBase` _avataractor)
          (:`then`
            (bind _asbp_weapon_base_2 (cast `/Game/RL/Weapon/BP_WeaponBase` _owneractor))
            (`/Game/RL/Weapon/BP_WeaponBase.SpawnBullet` :`self` _asbp_weapon_base_2 :`Transform` (`/Game/RL/AI/BP_MonsterBase.GetMonsterFirePosition` _asbp_monster_base) :`Container` (`BlueprintMapLibrary.Map_Find` (`self.EffectContainerMap`) (struct :`TagName` "Event.Shared.WeaponHit.Bullet")) :`Level` (`self.GetAbilityLevel`))
            (`|ExecutionSequence`
              (:`then_0`
                (bind (_returnvalue_location_2 _returnvalue_rotation_2) (`KismetMathLibrary.BreakTransform` (`/Game/RL/Weapon/BP_WeaponBase.GetMuzzleTransform` _asbp_weapon_base_2)))
                (`self.K2_AddGameplayCueWithParams` (struct :`TagName` "GameplayCue.BulletMuzzle.Default") (`AbilitySystemBlueprintLibrary.MakeGameplayCueParameters` 0.0 0.0 (struct) (struct) (struct) (struct) (struct) _returnvalue_location_2 (`KismetMathLibrary.Conv_RotatorToVector` _returnvalue_rotation_2) null _asbp_weapon_base_2))
                (goto _label))))
          (:`CastFailed`
            (`self.K2_EndAbility`)))))
    (else
      (`self.K2_EndAbility`))))

(event `self.K2_CommitExecute`)

(fn `K2_CanActivateAbility`
  (params (ActorInfo :type "GameplayAbilityActorInfo Structure") (Handle :type "GameplayAbilitySpecHandle Structure"))
  (returns (RelevantTags :type "GameplayTagContainer Structure") (ReturnValue :type Boolean))
  (return (struct) true))