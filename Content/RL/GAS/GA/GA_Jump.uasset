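; GA_Jump is a gameplay ability that moves the VR pawn along a precomputed jump path, optionally in bullet time.
; Activation applies a path-following root motion source from the pawn's jump data, starts bullet-time post-process and looping sound, and enters power-mode bullet time if the pawn's flag is set.
; A landed gameplay event spawns a foot impact effect and ends the ability, as does the bullet-time stop callback.
; Ending reverses the bullet-time state and effects.
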(event `OnBulletTimeStop`
  (`self.K2_EndAbility`))

(event `self.K2_ActivateAbility`
  (bind _returnvalue (subsystem `/Game/RL/Subsystem/BulletTimeManager/BP_BulletTimeManager`))
  (bind _vr_pawn (`self.VR Pawn`))
  (bind _vr_pawn_2 (`self.VR Pawn`))
  (bind (_bcanjump _jump_trace_path_potions _duration) (`/Game/RL/Core/BP_VR_Pawn.GetJumpData` _vr_pawn))
  (bind _charactermovement (`Character.CharacterMovement` _vr_pawn))
  (bind _returnvalue_2 (`self.K2_CommitAbility`))
  (if _returnvalue_2
    (bind _asbp_vr_pawn (cast `/Game/RL/Core/BP_VR_Pawn` (`self.GetAvatarActorFromActorInfo`)))
    (set `self.VR Pawn` _asbp_vr_pawn)
    (`|ExecutionSequence`
      (:`then_0`
        (if (`/Game/RL/Core/BP_VR_Pawn.bJumpEnterBulletTime` _vr_pawn_2)
          (`/Game/RL/Subsystem/BulletTimeManager/BP_BulletTimeManager.EnterPowerModeBulletTime` _returnvalue true)
          (add `/Game/RL/Subsystem/BulletTimeManager/BP_BulletTimeManager.BulletTimeStopHandler` _returnvalue (delegate `OnBulletTimeStop`))
          (`/Game/RL/Subsystem/BulletTimeManager/BP_BulletTimeManager.RemoveIgnoreActor` (subsystem `/Game/RL/Subsystem/BulletTimeManager/BP_BulletTimeManager`) _vr_pawn_2)))
      (:`then_1`
        (`/Game/RL/Subsystem/PostProcessManager/BP_PostProcessMgr.EnterEffect_BulletTime` (subsystem `/Game/RL/Subsystem/PostProcessManager/BP_PostProcessMgr`))
        (bind _returnvalue_3 (`GameplayStatics.SpawnSound2D` "/Game/RL/Sound/BulletTime/BulletTimeEnterAndLoop_Cue.BulletTimeEnterAndLoop_Cue" 1.0 1.0 0.0 null))
        (set `self.BulletTimeLoopSound` _returnvalue_3))
      (:`then_2`
        (`RMSLibrary.RemoveRootMotionSource` _charactermovement "Jump")
        (bind _output_get (set `self.Duration` _duration))
        (bind _output_get_2 (set `self.Jump Trace Path Potions` _jump_trace_path_potions))
        (`RMSLibrary.ApplyRootMotionSource_PathMoveToForce_V2` _charactermovement "Jump" (struct) _output_get_2 0 0.0 _output_get)
        (`AbilityTask_WaitGameplayEvent.WaitGameplayEvent` (struct :`TagName` "Event.Shared.OnLanded") (`self.VR Pawn`)
          (:`EventReceived`
            (`|ExecutionSequence`
              (:`then_0`
                (bind _vr_pawn_3 (`self.VR Pawn`)
                  (:`then`
                    (`NiagaraFunctionLibrary.SpawnSystemAtLocation` "/Game/ThirdParty/ProjectilesVol2/Effects/NS_Hit_20.NS_Hit_20" (`/Game/RL/Core/BP_PawnBase.GetFootLocation` _vr_pawn_3)))
                  (:`else`)))
              (:`then_1`
                (`self.K2_EndAbility`)))))))))

(event `self.K2_OnEndAbility`
  (params (bWasCancelled :type Boolean))
  (`|ExecutionSequence`
    (:`then_0`
      (bind _bullettimeloopsound (`self.BulletTimeLoopSound`)
        (:`then`
          (`AudioComponent.Stop` _bullettimeloopsound)
          (`ActorComponent.K2_DestroyComponent` _bullettimeloopsound))
        (:`else`)))
    (:`then_1`
      (`GameplayStatics.SpawnSound2D` "/Game/RL/Sound/BulletTime/QuitBulletTime_01_Cue.QuitBulletTime_01_Cue" 1.0 1.0 0.0 null)
      (`/Game/RL/Subsystem/PostProcessManager/BP_PostProcessMgr.QuitEffect_BulletTime` (subsystem `/Game/RL/Subsystem/PostProcessManager/BP_PostProcessMgr`)))
    (:`then_2`
      (bind _vr_pawn (`self.VR Pawn`)
        (:`then`
          (if (`/Game/RL/Core/BP_VR_Pawn.bJumpEnterBulletTime` _vr_pawn)
            (`/Game/RL/Subsystem/BulletTimeManager/BP_BulletTimeManager.QuitPowerModeBulletTime` (subsystem `/Game/RL/Subsystem/BulletTimeManager/BP_BulletTimeManager`))
            (`/Game/RL/Subsystem/BulletTimeManager/BP_BulletTimeManager.AddIgnoreActor` (subsystem `/Game/RL/Subsystem/BulletTimeManager/BP_BulletTimeManager`) (`self.GetAvatarActorFromActorInfo`))))
        (:`else`)))))