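; Post-process proxy that plays the bullet time, blood damage and death screen effects.
; BeginPlay creates a dynamic material per effect in a shared blendables array; UpdatePPMats copies it into the PostProcess settings whenever an effect toggles its weight.
; Timelines animate material parameters: bullet time and death reverse to exit, while blood restarts per hit, scaled by damage with a random offset.
; Death also quits bullet time; an older bullet-time implementation remains unconnected.
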(event `self.ReceiveBeginPlay`
  ;[1 1 1] Init
  (`|ExecutionSequence`
    (:`then_0`
      (bind _returnvalue (`KismetMaterialLibrary.CreateDynamicMaterialInstance` "/Game/RL/Subsystem/PostProcessManager/PPMatInst/M_PP_BulletTime_Boom_Inst.M_PP_BulletTime_Boom_Inst"))
      (bind _returnvalue_2 (`KismetArrayLibrary.Array_Add` (`self.Mats_WeightedBlendable`) (make `WeightedBlendable` -1.0 _returnvalue)))
      (set `self.Mat_BulletTime` (make `/Game/RL/Subsystem/PostProcessManager/SPostProcessMatInfo` _returnvalue_2 _returnvalue)))
    (:`then_1`
      (bind _returnvalue_3 (`KismetMaterialLibrary.CreateDynamicMaterialInstance` "/Game/RL/Mat/PostProcess/M_PP_Blooding.M_PP_Blooding"))
      (bind _returnvalue_4 (`KismetArrayLibrary.Array_Add` (`self.Mats_WeightedBlendable`) (make `WeightedBlendable` -1.0 _returnvalue_3)))
      (set `self.Mat_Blooding` (make `/Game/RL/Subsystem/PostProcessManager/SPostProcessMatInfo` _returnvalue_4 _returnvalue_3)))
    (:`then_2`
      (bind _returnvalue_5 (`KismetMaterialLibrary.CreateDynamicMaterialInstance` "/Game/RL/Subsystem/PostProcessManager/PPMatInst/M_PP_Death_Inst.M_PP_Death_Inst"))
      (bind _returnvalue_6 (`KismetArrayLibrary.Array_Add` (`self.Mats_WeightedBlendable`) (make `WeightedBlendable` -1.0 _returnvalue_5)))
      (set `self.MatDeath` (make `/Game/RL/Subsystem/PostProcessManager/SPostProcessMatInfo` _returnvalue_6 _returnvalue_5)))))

(event `EnterEffect_BulletTime`
  (bind (_mat_bullettime_id _mat_bullettime_mat) (break `/Game/RL/Subsystem/PostProcessManager/SPostProcessMatInfo` (`self.Mat_BulletTime`)))
  (bind (_mat_bullettime_id_2 _mat_bullettime_mat_2) (break `/Game/RL/Subsystem/PostProcessManager/SPostProcessMatInfo` (`self.Mat_BulletTime`)))
  (bind (_mat_bullettime_id_3 _mat_bullettime_mat_3) (break `/Game/RL/Subsystem/PostProcessManager/SPostProcessMatInfo` (`self.Mat_BulletTime`)))
  (bind (_mat_bullettime_id_4 _mat_bullettime_mat_4) (break `/Game/RL/Subsystem/PostProcessManager/SPostProcessMatInfo` (`self.Mat_BulletTime`)))
  (bind (_id _mat) (break `/Game/RL/Subsystem/PostProcessManager/SPostProcessMatInfo` (`self.Mat_BulletTime`)))
  (`KismetArrayLibrary.Array_Set` (`self.Mats_WeightedBlendable`) _id (make `WeightedBlendable` 1.0 _mat))
  (`self.UpdatePPMats`)
  (bind (_direction _liner) (`Timeline|BulletTime_Boom` :!label _label)
    (:`Update`
      (`|ExecutionSequence`
        (:`then_0`
          (`MaterialInstanceDynamic.SetScalarParameterValue` _mat_bullettime_mat "Desaturation" (`KismetMathLibrary.Lerp` 0.0 0.5 _liner)))
        (:`then_1`
          (`MaterialInstanceDynamic.SetScalarParameterValue` _mat_bullettime_mat_3 "DarkConerStrength" (`KismetMathLibrary.Lerp` 0.0 0.8 _liner)))
        (:`then_2`
          (if (`|EnumEquality` _direction "Forward")
            (`MaterialInstanceDynamic.SetScalarParameterValue` _mat_bullettime_mat_4 "BoomTime" _liner)))))
    (:`Finished`
      (if (`|EnumEquality` _direction "Backward")
        (`KismetArrayLibrary.Array_Set` (`self.Mats_WeightedBlendable`) _mat_bullettime_id_2 (make `WeightedBlendable` -1.0 _mat_bullettime_mat_2))
        (`self.UpdatePPMats`)))))

(event `QuitEffect_BulletTime`
  (goto _label :!via `Reverse`))

(event `EnterEffect_Blooding`
  (params (DamageDegree :type "Float (double-precision)" :default 0.5))
  (bind _returnvalue (`KismetMathLibrary.RandomFloat`))
  (bind (_mat_blooding_id _mat_blooding_mat) (break `/Game/RL/Subsystem/PostProcessManager/SPostProcessMatInfo` (`self.Mat_Blooding`)))
  (bind (_mat_blooding_id_2 _mat_blooding_mat_2) (break `/Game/RL/Subsystem/PostProcessManager/SPostProcessMatInfo` (`self.Mat_Blooding`)))
  (bind (_mat_blooding_id_3 _mat_blooding_mat_3) (break `/Game/RL/Subsystem/PostProcessManager/SPostProcessMatInfo` (`self.Mat_Blooding`)))
  (bind (_mat_blooding_id_4 _mat_blooding_mat_4) (break `/Game/RL/Subsystem/PostProcessManager/SPostProcessMatInfo` (`self.Mat_Blooding`)))
  (bind (_mat_blooding_id_5 _mat_blooding_mat_5) (break `/Game/RL/Subsystem/PostProcessManager/SPostProcessMatInfo` (`self.Mat_Blooding`)))
  (bind (_id _mat) (break `/Game/RL/Subsystem/PostProcessManager/SPostProcessMatInfo` (`self.Mat_Blooding`)))
  (set `self.Damage Degree` (`KismetMathLibrary.Lerp` 0.2 1.0 (`KismetMathLibrary.FClamp` DamageDegree)))
  (`KismetArrayLibrary.Array_Set` (`self.Mats_WeightedBlendable`) _id (make `WeightedBlendable` 1.0 _mat))
  (`self.UpdatePPMats`)
  (`|ExecutionSequence`
    (:`then_0`
      (`MaterialInstanceDynamic.SetScalarParameterValue` _mat_blooding_mat_3 "Degree" (`self.Damage Degree`)))
    (:`then_1`
      (`MaterialInstanceDynamic.SetVectorParameterValue` _mat_blooding_mat_2 "RandomOffset" (make `LinearColor` _returnvalue _returnvalue 0.0 1.0)))
    (:`then_2`
      (bind (_direction _liner) (`Timeline|Timeline_Blooding` :!via `PlayFromStart`)
        (:`Update`
          (`|ExecutionSequence`
            (:`then_0`
              (`MaterialInstanceDynamic.SetScalarParameterValue` _mat_blooding_mat_4 "BloodPower" (* _liner (`KismetMathLibrary.Lerp` 3.0 5.0 (`self.Damage Degree`)))))
            (:`then_1`
              (`MaterialInstanceDynamic.SetScalarParameterValue` _mat_blooding_mat "MinIntensity" (* _liner 0.5)))))
        (:`Finished`
          (`KismetArrayLibrary.Array_Set` (`self.Mats_WeightedBlendable`) _mat_blooding_id_5 (make `WeightedBlendable` -1.0 _mat_blooding_mat_5))
          (`self.UpdatePPMats`))))))

(event `EnterEffect_Death`
  (bind (_matdeath_id _matdeath_mat) (break `/Game/RL/Subsystem/PostProcessManager/SPostProcessMatInfo` (`self.MatDeath`)))
  (bind (_matdeath_id_2 _matdeath_mat_2) (break `/Game/RL/Subsystem/PostProcessManager/SPostProcessMatInfo` (`self.MatDeath`)))
  (bind (_id _mat) (break `/Game/RL/Subsystem/PostProcessManager/SPostProcessMatInfo` (`self.MatDeath`)))
  (`|ExecutionSequence`
    (:`then_0`
      (`self.QuitEffect_BulletTime`))
    (:`then_1`
      (`KismetArrayLibrary.Array_Set` (`self.Mats_WeightedBlendable`) _id (make `WeightedBlendable` 1.0 _mat))
      (`self.UpdatePPMats`)
      (bind (_direction _liner) (`Timeline|Timeline_Dead` :!label _label_2)
        (:`Update`
          (`MaterialInstanceDynamic.SetScalarParameterValue` _matdeath_mat "Desaturation" _liner))
        (:`Finished`
          (if (`|EnumEquality` _direction "Backward")
            (`KismetArrayLibrary.Array_Set` (`self.Mats_WeightedBlendable`) _matdeath_id_2 (make `WeightedBlendable` -1.0 _matdeath_mat_2))
            (`self.UpdatePPMats`)))))))

(event `QuitEffect_Death`
  (goto _label_2 :!via `Reverse`))

(fn `UpdatePPMats`
  (setmembers `PostProcessSettings` :`StructRef` (`PostProcessComponent.Settings` (`self.PostProcess`)) :`WeightedBlendables` (make `WeightedBlendables` (`self.Mats_WeightedBlendable`))))

(fn `UserConstructionScript`)