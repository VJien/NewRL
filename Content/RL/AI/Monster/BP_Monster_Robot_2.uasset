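; BP_Monster_Robot_2 is a monster robot Blueprint that disintegrates visually when it dies.
; On BeginPlay it creates a dynamic instance of DistMat and applies it to the mesh's first material slot.
; DoDeath runs the parent death logic, activates the NSMeshDisintegration effect and plays a timeline.
; That timeline drives an Erode value into both the material and the effect, keeping dissolve and particles in sync.
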(event `self.ReceiveBeginPlay`
  (`parent.ReceiveBeginPlay`)
  (bind _returnvalue (`KismetMaterialLibrary.CreateDynamicMaterialInstance` (`self.DistMat`)))
  (bind _output_get (set `self.BodyMatInstance` _returnvalue))
  (`PrimitiveComponent.SetMaterial` (`self.Mesh`) 0 _output_get))

(event `/Game/RL/Core/BP_PawnBase.DoDeath`
  (params (SourceASC :type "FGComponent Object Reference") (Damage :type "Float (single-precision)") (HitResult :type "HitResult Structure"))
  (`parent.DoDeath` SourceASC Damage HitResult)
  (`ActorComponent.SetActive` (`self.NS_MeshDisintegration`) true false)
  (bind (_direction _erode) (`Timeline|Timeline_0`)
    (:`Update`
      (`MaterialInstanceDynamic.SetScalarParameterValue` (`self.BodyMatInstance`) "Erode" _erode)
      (`NiagaraComponent.SetVariableFloat` (`self.NS_MeshDisintegration`) "Erode" _erode))))

(fn `UserConstructionScript`
  (`parent.UserConstructionScript`))