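; BP_PostProcessMgr is a manager that exposes gameplay screen effects for bullet time, bleeding and death.
; On init it reuses the first BP_PostProcessProxy actor in the level, or spawns one if none exists.
; Effect events forward directly to that proxy, with bleeding passing a damage degree.
; A separate event registers the proxy with the bullet time manager as an ignored actor.
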(event `self.OnInit`
  (bind _outactors (`GameplayStatics.GetAllActorsOfClass` "/Game/RL/Subsystem/PostProcessManager/BP_PostProcessProxy.BP_PostProcessProxy_C"))
  (if (> (`KismetArrayLibrary.Array_Length` _outactors) 0)
    (set `self.PostProcessProxy` (`|GetArrayItem` _outactors))
    (else
      (bind _returnvalue (`|SpawnActorFromClass` "/Game/RL/Subsystem/PostProcessManager/BP_PostProcessProxy.BP_PostProcessProxy_C" (`KismetMathLibrary.MakeTransform` (0.0 0.0 0.0)) "Undefined" "OverrideRootScale" null null))
      (set `self.PostProcessProxy` _returnvalue))))

(event `IgnoreBulletTime`
  (`/Engine/EditorBlueprintResources/StandardMacros.IsValid` (`self.PostProcessProxy`)
    (:`Is Valid`
      (`/Game/RL/Subsystem/BulletTimeManager/BP_BulletTimeManager.AddIgnoreActor` (subsystem `/Game/RL/Subsystem/BulletTimeManager/BP_BulletTimeManager`) (`self.PostProcessProxy`)))))

(event `self.OnTick`
  (params (DeltaTime :type "Float (single-precision)")))

(event `EnterEffect_BulletTime`
  (`/Game/RL/Subsystem/PostProcessManager/BP_PostProcessProxy.EnterEffect_BulletTime` (`self.PostProcessProxy`)))

(event `QuitEffect_BulletTime`
  (`/Game/RL/Subsystem/PostProcessManager/BP_PostProcessProxy.QuitEffect_BulletTime` (`self.PostProcessProxy`)))

(event `EnterEffect_Blooding`
  (params (DamageDegree :type "Float (double-precision)" :default 0.5))
  (`/Game/RL/Subsystem/PostProcessManager/BP_PostProcessProxy.EnterEffect_Blooding` (`self.PostProcessProxy`) DamageDegree))

(event `EnterEffect_Death`
  (`/Game/RL/Subsystem/PostProcessManager/BP_PostProcessProxy.EnterEffect_Death` (`self.PostProcessProxy`)))

(event `QuitEffect_Death`
  (`/Game/RL/Subsystem/PostProcessManager/BP_PostProcessProxy.QuitEffect_Death` (`self.PostProcessProxy`)))