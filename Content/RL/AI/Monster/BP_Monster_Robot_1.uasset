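; Robot monster Blueprint that adds an erode disintegration effect on death to its parent monster logic.
; On BeginPlay it creates a dynamic instance of the robot body material and applies it to the mesh.
; DoDeath activates a Niagara mesh disintegration system and plays an Erode timeline that drives the same Erode value into both the material and the particles, keeping them in sync.
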(event `self.ReceiveBeginPlay`
  (`parent.ReceiveBeginPlay`)
  (bind _returnvalue (`KismetMaterialLibrary.CreateDynamicMaterialInstance` "/Game/RL/Effects/BodyDisintegration/Robot3_SmoothBody_Dist_Inst.Robot3_SmoothBody_Dist_Inst"))
  (bind _output_get (set `self.BodyMat` _returnvalue))
  (`PrimitiveComponent.SetMaterial` (`self.Mesh`) 0 _output_get))

(event `self.ReceiveTick`
  (params (DeltaSeconds :type "Float (single-precision)"))
  (`parent.ReceiveTick` DeltaSeconds))

(event `/Game/RL/Core/BP_PawnBase.DoDeath`
  (params (SourceASC :type "FGComponent Object Reference") (Damage :type "Float (single-precision)") (HitResult :type "HitResult Structure"))
  (`parent.DoDeath` SourceASC Damage HitResult)
  (`ActorComponent.SetActive` (`self.NS_MeshDisintegration`) true false)
  (bind (_direction _erode) (`Timeline|Erode`)
    (:`Update`
      (`MaterialInstanceDynamic.SetScalarParameterValue` (`self.BodyMat`) "Erode" _erode)
      (`NiagaraComponent.SetVariableFloat` (`self.NS_MeshDisintegration`) "Erode" _erode))))

(fn `UserConstructionScript`
  (`parent.UserConstructionScript`))