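; Explosive scene item that is visible and has query collision only during bullet time, checked every tick.
; Point damage lowers its health, and at zero it explodes, damaging pawns overlapping a radius-sized sphere.
; Damage goes through GAS as a caller-set physical damage gameplay effect.
; The blast spawns optional Niagara, particle and sound effects, then hides the mesh and expires shortly after.
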(event `self.ReceiveTick`
  (params (DeltaSeconds :type "Float (single-precision)"))
  (bind _sphere (`self.Sphere`))
  (bind _returnvalue (`/Game/RL/Subsystem/BulletTimeManager/BP_BulletTimeManager.IsInBulletTime` (subsystem `/Game/RL/Subsystem/BulletTimeManager/BP_BulletTimeManager`) self))
  (`SceneComponent.SetVisibility` _sphere _returnvalue false)
  (`SceneComponent.SetVisibility` (`self.StaticMesh`) _returnvalue false)
  (`PrimitiveComponent.SetCollisionEnabled` _sphere (select `bool` _returnvalue :`false` "NoCollision" :`true` "QueryOnly" :!type "ECollisionEnabled Enum"))
  (`PrimitiveComponent.SetCollisionEnabled` (`self.StaticMesh`) (select `bool` _returnvalue :`false` "NoCollision" :`true` "QueryOnly" :!type "ECollisionEnabled Enum")))

(event `/Game/RL/Interface/BPI_Damage.TakePointDamage`
  (params (Damage :type "Float (single-precision)") (Causer :type "Actor Object Reference") (Instigator :type "Actor Object Reference") (HitResult :type "HitResult Structure") (DamageType :type "DamageType Class Reference"))
  (bind _output_get (set `self.Health` (`KismetMathLibrary.FTrunc` (- (`KismetMathLibrary.Conv_IntToDouble` (`self.Health`)) Damage))))
  (if (<= _output_get 0)
    (`self.Explode`)))

(event `self.ReceiveAnyDamage`
  (params (Damage :type "Float (single-precision)") (DamageType :type "DamageType Object Reference") (InstigatedBy :type "Controller Object Reference") (DamageCauser :type "Actor Object Reference")))

(fn `Explode`
  (locals (AllPanws :type "Array of Actor Object Reference"))
  (bind _returnvalue (`self.K2_GetActorLocation`))
  (bind _output_get (set `local.AllPanws` (`PrimitiveComponent.GetOverlappingActors` (`self.Sphere`) "/Game/RL/Core/BP_PawnBase.BP_PawnBase_C")))
  (for _array_element _output_get
    (`/Engine/EditorBlueprintResources/StandardMacros.IsValid` _array_element
      (:`Is Valid`
        (bind _returnvalue_2 (`AbilitySystemBlueprintLibrary.GetAbilitySystemComponent` _array_element))
        (`/Engine/EditorBlueprintResources/StandardMacros.IsValid` _returnvalue_2
          (:`Is Valid`
            (`/Game/RL/FunctionLib/FLib_Utility.ApplyByCallerGameplayEffect` _returnvalue_2 (struct :`TagName` "Attribute.Damage.Physics") "/FastGas/GE/ByCaller/GE_Override_Damage_Physics.GE_Override_Damage_Physics_C" 0.0 (struct) (`self.Damage`)))))))
  (`|ExecutionSequence`
    (:`then_0`
      (bind _ns_explode (`self.NS_Explode`)
        (:`then`
          (`NiagaraFunctionLibrary.SpawnSystemAtLocation` _ns_explode _returnvalue))
        (:`else`)))
    (:`then_1`
      (bind _fx_explode (`self.FX_Explode`)
        (:`then`
          (`GameplayStatics.SpawnEmitterAtLocation` _fx_explode _returnvalue))
        (:`else`)))
    (:`then_2`
      (bind _sound_explode (`self.Sound_Explode`)
        (:`then`
          (`GameplayStatics.SpawnSoundAtLocation` _sound_explode _returnvalue (struct) 1.0 1.0 0.0 null null))
        (:`else`)))
    (:`then_3`
      (`PrimitiveComponent.SetCollisionEnabled` (`self.Sphere`) "NoCollision")
      (`SceneComponent.SetVisibility` (`self.StaticMesh`) false false)
      (`self.SetLifeSpan` 0.2))))

(fn `UserConstructionScript`
  (`SphereComponent.SetSphereRadius` (`self.Sphere`) (`self.Radius`) true))