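; BP_3DUI_Container is a container that hosts UI in the 3D scene through its Widget component.
; On BeginPlay it constructs a controller for each UIClass entry, initializes it with itself, registers it with BPEventSystem and stores it in WidgetsController.
; It then displays only the first controller's widget.
; SendUIMessage forwards messages to BPEventSystem, while PushNextUI and PopNowUI are empty stubs.
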(event `self.ReceiveBeginPlay`
  (bind _output (`|GetArrayItem` (`self.WidgetsController`)))
  (`|ExecutionSequence`
    (:`then_0`
      (for _array_element (`self.UIClass`)
        (bind _returnvalue (`|GenericCreateObject` _array_element self))
        (`|ExecutionSequence`
          (:`then_0`
            (`/Game/RL/Widget/UWController/Obj_BaseUI.OnInit` _returnvalue self))
          (:`then_1`
            (`/Game/RL/Subsystem/EventSystem/BP_EventSystem.RegisterUIEvent` (subsystem `/Game/RL/Subsystem/EventSystem/BP_EventSystem`) _returnvalue))
          (:`then_2`
            (`KismetArrayLibrary.Array_Add` (`self.WidgetsController`) _returnvalue)))))
    (:`then_1`
      (`/Engine/EditorBlueprintResources/StandardMacros.IsValid` _output
        (:`Is Valid`
          (`WidgetComponent.SetWidget` (`self.Widget`) (`/Game/RL/Widget/UWController/Obj_BaseUI.GetWidget` _output)))))))

(fn `PopNowUI`)

(fn `PushNextUI`
  (params (UW :type "UserWidget Class Reference")))

(fn `SendUIMessage`
  (params (UIMessage :type "/Game/RL/Subsystem/EventSystem/UIEvent/S_UIMessage Structure (by ref)"))
  (`/Game/RL/Subsystem/EventSystem/BP_EventSystem.SendUIMessage` (subsystem `/Game/RL/Subsystem/EventSystem/BP_EventSystem`) UIMessage))

(fn `UserConstructionScript`)