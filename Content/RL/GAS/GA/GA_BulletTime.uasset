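; GA_BulletTime is a Gameplay Ability that runs the player-facing bullet time power mode.
; On successful commit it starts bullet time through BPBulletTimeManager, spawns the looping sound and enables the post-process effect.
; The manager's stop callback ends the ability, which then stops the loop, plays the exit sound and removes the effect.
; An older self-managed energy and exit-event path is left unconnected.
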(event `OnBulletTimeStop`
  (`self.K2_EndAbility`))

(event `self.K2_ActivateAbility`
  (bind _returnvalue (subsystem `/Game/RL/Subsystem/BulletTimeManager/BP_BulletTimeManager`))
  (bind _returnvalue_2 (`self.K2_CommitAbility`))
  (if _returnvalue_2
    (set `self.bHasEnter` true)
    (`|ExecutionSequence`
      (:`then_0`
        ;[1 1 1] 调用子弹时间系统
        (`/Game/RL/Subsystem/BulletTimeManager/BP_BulletTimeManager.EnterPowerModeBulletTime` _returnvalue false)
        (bind _returnvalue_3 (`GameplayStatics.SpawnSound2D` "/Game/RL/Sound/BulletTime/BulletTimeEnterAndLoop_Cue.BulletTimeEnterAndLoop_Cue" 1.0 1.0 0.0 null))
        (set `self.BulletTimeLoopSound` _returnvalue_3)
        (add `/Game/RL/Subsystem/BulletTimeManager/BP_BulletTimeManager.BulletTimeStopHandler` _returnvalue (delegate `OnBulletTimeStop`)))
      (:`then_1`
        (`/Game/RL/Subsystem/PostProcessManager/BP_PostProcessMgr.EnterEffect_BulletTime` (subsystem `/Game/RL/Subsystem/PostProcessManager/BP_PostProcessMgr`))))
    (else
      (`self.K2_EndAbility`))))

(event `self.K2_OnEndAbility`
  (params (bWasCancelled :type Boolean))
  (if (`self.bHasEnter`)
    (`|ExecutionSequence`
      (:`then_0`
        (bind _bullettimeloopsound (`self.BulletTimeLoopSound`)
          (:`then`
            (`AudioComponent.Stop` _bullettimeloopsound)
            (`ActorComponent.K2_DestroyComponent` _bullettimeloopsound))
          (:`else`)))
      (:`then_1`
        (`GameplayStatics.SpawnSound2D` "/Game/RL/Sound/BulletTime/QuitBulletTime_01_Cue.QuitBulletTime_01_Cue" 1.0 1.0 0.0 null))
      (:`then_2`
        (`/Game/RL/Subsystem/PostProcessManager/BP_PostProcessMgr.QuitEffect_BulletTime` (subsystem `/Game/RL/Subsystem/PostProcessManager/BP_PostProcessMgr`))))))