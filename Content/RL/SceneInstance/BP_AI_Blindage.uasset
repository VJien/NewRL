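; AI cover point (blindage) that tracks an occupant and keeps a per-monster weight.
; On a randomized delay it rescores registered monsters: bonuses for being in player view, near 700 units from the player, and having a short nav path here; overly long paths score zero.
; An optional DependOnActor gates scoring and occupancy; its destruction blackens the marker.
; Debug mode shows the occupancy-colored sphere and camera-facing weight text.
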(event `self.ReceiveBeginPlay`
  (`|ExecutionSequence`
    (:`then_0`
      (bind _returnvalue (`KismetMaterialLibrary.CreateDynamicMaterialInstance` "/Game/RL/Mat/M_Ghost_Blindage.M_Ghost_Blindage"))
      (bind _output_get (set `self.Mat` _returnvalue))
      (`PrimitiveComponent.SetMaterial` (`self.Sphere`) 0 _output_get)
      (`self.SetOccupant` null)
      (if (`self.bDebug`)
        (`SceneComponent.SetVisibility` (`self.Sphere`) true true)
        (else
          (`SceneComponent.SetVisibility` (`self.Sphere`) false true))))
    (:`then_1`
      (bind _dependonactor (`self.DependOnActor`)
        (:`then`
          (set `self.bIsDependOnActor` true)
          (add `self.OnDestroyed` _dependonactor (delegate `OnDepandActorDestroy`)))
        (:`else`
          (set `self.bIsDependOnActor` false))))
    (:`then_2`
      (set `self.UpdateDelta` (`KismetMathLibrary.RandomFloatInRange` 1.0 2.0)))))

(event `OnDepandActorDestroy` :!signature `self.OnDestroyed`
  (params (DestroyedActor :type "Actor Object Reference"))
  (`MaterialInstanceDynamic.SetVectorParameterValue` :`self` (`self.Mat`) :`ParameterName` "Color"))

(event `self.ReceiveTick`
  (params (DeltaSeconds :type "Float (single-precision)"))
  (bind _allmonsters (`self.AllMonsters`))
  (`|ExecutionSequence`
    (:`then_0`
      (if (`self.bDebug`)
        (set `self.WeightInfo` "")
        (bind _keys (`BlueprintMapLibrary.Map_Keys` _allmonsters))
        (for _array_element _keys
          (set `self.WeightInfo` (`KismetStringLibrary.Concat_StrStr` (`self.WeightInfo`) (`KismetStringLibrary.Concat_StrStr` (`KismetSystemLibrary.GetDisplayName` _array_element) " =  " (`KismetStringLibrary.Conv_DoubleToString` (`BlueprintMapLibrary.Map_Find` _allmonsters _array_element)) " \n"))))
        (`TextRenderComponent.K2_SetText` (`self.TextRender`) (`KismetTextLibrary.Conv_StringToText` (`self.WeightInfo`)))
        (`SceneComponent.K2_SetWorldRotation` (`self.TextRender`) (`KismetMathLibrary.FindLookAtRotation` (`SceneComponent.K2_GetComponentLocation` (`self.TextRender`)) (`self.K2_GetActorLocation` (`GameplayStatics.GetPlayerCameraManager` 0))) false false)))
    (:`then_1`
      (`KismetSystemLibrary.Delay` (`self.UpdateDelta`))
      (bind _keys_2 (`BlueprintMapLibrary.Map_Keys` (`self.AllMonsters`)))
      (for _array_element_2 _keys_2
        (bind _asbp_pawn_base (cast `/Game/RL/Core/BP_PawnBase` (`GameplayStatics.GetPlayerPawn` 0)))
        (`self.Update Weight` _array_element_2 _asbp_pawn_base)))))

(fn `BP_AI_Blindage_AutoGenFunc`
  (params (DestroyedActor :type "Actor Object Reference"))
  (bind _asbp_monster_base (cast `/Game/RL/AI/BP_MonsterBase` DestroyedActor))
  (clear `self.OnDestroyed` _asbp_monster_base)
  (`BlueprintMapLibrary.Map_Remove` (`self.AllMonsters`) _asbp_monster_base))

(fn `GetOccupant`
  (returns (Occupant :type "/Game/RL/AI/BP_MonsterBase Object Reference"))
  (return (`self.Occupant`)))

(fn `GetWeight`
  (params (Monster :type "/Game/RL/AI/BP_MonsterBase Object Reference (by ref)"))
  (returns (Value :type "Float (double-precision)"))
  (return (`BlueprintMapLibrary.Map_Find` (`self.AllMonsters`) Monster)))

(fn `InPlayerFov`
  (params (Monster :type "Actor Object Reference"))
  (returns (ReturnValue :type Boolean))
  (bind _returnvalue (`GameplayStatics.GetPlayerCameraManager` 0))
  (`/Engine/EditorBlueprintResources/StandardMacros.IsValid` _returnvalue
    (:`Is Valid`
      (return (> (`KismetMathLibrary.Dot_VectorVector` (`KismetMathLibrary.Normal` (`KismetMathLibrary.GetForwardVector` (`PlayerCameraManager.GetCameraRotation` _returnvalue))) (`KismetMathLibrary.Normal` (- (`self.K2_GetActorLocation` Monster) (`PlayerCameraManager.GetCameraLocation` _returnvalue)))) (`KismetMathLibrary.DegCos` (* (`PlayerCameraManager.GetFOVAngle` _returnvalue) 0.5)))))))

(fn `IsOccupied`
  (returns (bIsOccupied :type Boolean))
  (return (`KismetSystemLibrary.IsValid` (`self.Occupant`))))

(fn `RegisterMonster`
  (params (Monster :type "/Game/RL/AI/BP_MonsterBase Object Reference"))
  (`BlueprintMapLibrary.Map_Add` (`self.AllMonsters`) Monster)
  (add `self.OnDestroyed` Monster (`|CreateDelegate` :!event `BP_AI_Blindage_AutoGenFunc`)))

(fn `SetOccupant`
  (params (Occupant :type "/Game/RL/AI/BP_MonsterBase Object Reference"))
  (if (`self.bIsDependOnActor`)
    (`self.DependOnActor`
      (:`then`
        _)
      (:`else`)))
  (bind _output_get (set `self.Occupant` Occupant))
  (`MaterialInstanceDynamic.SetVectorParameterValue` (`self.Mat`) "Color" (select `bool` (`KismetSystemLibrary.IsValid` _output_get) :`false` (struct :`R` 0.02254 :`G` 1.0 :`A` 1.0) :`true` (struct :`R` 1.0 :`G` 0.014042 :`A` 1.0) :!type "LinearColor Structure")))

(fn `Update Weight`
  (params (Monster :type "/Game/RL/AI/BP_MonsterBase Object Reference") (TargetPlayer :type "/Game/RL/Core/BP_PawnBase Object Reference"))
  (locals (outWeight :type "Float (double-precision)" :default 0.0))
  (bind _newvar_0 (`self.NewVar_0`))
  (bind _newvar_0_2 (`self.NewVar_0`))
  (bind _pathcost (`NavigationSystemV1.GetPathCost` (`/Game/RL/Core/BP_PawnBase.GetFootLocation` Monster) (`NavigationSystemV1.K2_ProjectPointToNavigation` (`self.K2_GetActorLocation`) null null (50.0 50.0 50.0)) null null))
  (if (`self.bIsDependOnActor`)
    (`/Engine/EditorBlueprintResources/StandardMacros.IsValid` (`self.DependOnActor`)
      (:`Is Valid`
        _)
      (:`Is Not Valid`
        (`BlueprintMapLibrary.Map_Add` (`self.AllMonsters`) Monster)
        (return))))
  (`|ExecutionSequence`
    (:`then_0`
      (if (`self.InPlayerFov` Monster)
        (set `local.outWeight` (+ (`local.outWeight`) 0.5))))
    (:`then_1`
      (set `local.outWeight` (+ (`local.outWeight`) (`KismetMathLibrary.Lerp` 1.0 0.0 (`KismetMathLibrary.FClamp` (/ (`KismetMathLibrary.Abs` (- (`self.GetDistanceTo` Monster TargetPlayer) 700.0)) 700.0))))))
    (:`then_2`
      (if (> _pathcost 3000.0)
        (`BlueprintMapLibrary.Map_Add` (`self.AllMonsters`) (`local.Monster`))
        (`KismetSystemLibrary.PrintString` "Update Monster Weight" false false)
        (`/Engine/EditorBlueprintResources/StandardMacros.IncrementInt` _newvar_0
          (:`  `
            (`KismetSystemLibrary.PrintString` (`KismetStringLibrary.Conv_IntToString` _newvar_0) false false)
            (return)))
        (else
          (set `local.outWeight` (+ (`local.outWeight`) (`KismetMathLibrary.Lerp` 2.0 0.0 (`KismetMathLibrary.FClamp` (/ _pathcost 3000.0)))))
          (`BlueprintMapLibrary.Map_Add` (`self.AllMonsters`) (`local.Monster`) (`local.outWeight`))
          (`/Engine/EditorBlueprintResources/StandardMacros.IncrementInt` _newvar_0_2
            (:`  `
              (`KismetSystemLibrary.PrintString` (`KismetStringLibrary.Conv_IntToString` _newvar_0_2) false false)
              (`KismetSystemLibrary.PrintString` "Update Monster Weight" false false)
              (return))))))))

(fn `UserConstructionScript`)