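; Robot boss monster Blueprint that adds delayed shield regeneration and its own bullet-time rate on top of its parent monster class.
; On BeginPlay it registers with the bullet-time manager as an actor with a specified time rate.
; Taking damage removes active shield-regen effects and restarts a short timer, which reapplies the boss's shield-regen GameplayEffect when it expires.
; The construction script makes the Clock component follow the main mesh's pose through master pose.
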(event `self.ReceiveBeginPlay`
  (`parent.ReceiveBeginPlay`)
  (`/Game/RL/Subsystem/BulletTimeManager/BP_BulletTimeManager.AddSpecifyActor` (subsystem `/Game/RL/Subsystem/BulletTimeManager/BP_BulletTimeManager`) self 0.5))

(event `self.ReceiveTick`
  (params (DeltaSeconds :type "Float (single-precision)"))
  (`parent.ReceiveTick` DeltaSeconds))

(event `PostDamage_1`
  (params (SourceASC :type "FGComponent Object Reference") (Damage :type "Float (double-precision)") (HitResult :type "HitResult Structure"))
  (`KismetSystemLibrary.K2_ClearTimer` null "HealthRegenRestart")
  (`KismetSystemLibrary.K2_SetTimerDelegate` (delegate `HealthRegenRestart`) 2.0)
  (`AbilitySystemComponent.RemoveActiveEffectsWithTags` (`self.AbilitySystemComponent`) (struct :`GameplayTags` (struct :`(TagName` "State.Regen.Shield")))))

(event `HealthRegenRestart`
  (bind _abilitysystemcomponent (`self.AbilitySystemComponent`))
  (`AbilitySystemComponent.BP_ApplyGameplayEffectSpecToSelf` _abilitysystemcomponent (`AbilitySystemComponent.MakeOutgoingSpec` :`self` _abilitysystemcomponent :`GameplayEffectClass` "/Game/RL/GAS/GE/Regen/GE_Regen_Shield_Boss1.GE_Regen_Shield_Boss1_C")))

(fn `UserConstructionScript`
  (`parent.UserConstructionScript`)
  (`SkinnedMeshComponent.SetLeaderPoseComponent` (`self.Clock`) (`self.Mesh`) false))