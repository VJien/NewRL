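; Actor component that registers its owner with the bullet time manager to control how bullet time affects that actor.
; On BeginPlay it either adds the owner as an ignored actor or, if the specified rate is below 1.0, registers it with that custom time rate.
; On EndPlay it removes the owner from both the ignore and specified-rate lists.
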(event `self.ReceiveBeginPlay`
  (if (`self.IgnoreBulletTime`)
    (`/Game/RL/Subsystem/BulletTimeManager/BP_BulletTimeManager.AddIgnoreActor` (subsystem `/Game/RL/Subsystem/BulletTimeManager/BP_BulletTimeManager`) (`self.GetOwner`))
    (elif (< (`self.SpecifyBulletTimeRate`) 1.0)
      (`/Game/RL/Subsystem/BulletTimeManager/BP_BulletTimeManager.AddSpecifyActor` (subsystem `/Game/RL/Subsystem/BulletTimeManager/BP_BulletTimeManager`) (`self.GetOwner`) (`self.SpecifyBulletTimeRate`)))))

(event `self.ReceiveEndPlay`
  (params (EndPlayReason :type "EEndPlayReason Enum" :default "Destroyed"))
  (`/Game/RL/Subsystem/BulletTimeManager/BP_BulletTimeManager.RemoveSpecifyActor` (subsystem `/Game/RL/Subsystem/BulletTimeManager/BP_BulletTimeManager`) (`self.GetOwner`))
  (`/Game/RL/Subsystem/BulletTimeManager/BP_BulletTimeManager.RemoveIgnoreActor` (subsystem `/Game/RL/Subsystem/BulletTimeManager/BP_BulletTimeManager`) (`self.GetOwner`)))