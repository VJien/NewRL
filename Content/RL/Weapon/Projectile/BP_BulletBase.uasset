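; Base bullet projectile that flies forward at a set speed, with its body effect assigned at construction.
; Each tick it sphere-traces from its last location to the current one instead of using collision events, skipping ignored actors.
; Living enemy pawns and non-pawn actors receive a GAS hit event to the instigator plus point damage; other pawns receive neither.
; Any such hit, or damage to the bullet, calls the empty OnHit hook and destroys it.
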(event `self.ReceiveBeginPlay`
  (`parent.ReceiveBeginPlay`)
  (set `MovementComponent.Velocity` (* (`self.GetActorForwardVector`) (`self.Speed`)) (`self.ProjectileMovement`))
  (set `self.LastLoc` (`self.K2_GetActorLocation`)))

(event `self.Sphere.OnComponentBeginOverlap`
  (params (OverlappedComponent :type "PrimitiveComponent Object Reference") (OtherActor :type "Actor Object Reference") (OtherComp :type "PrimitiveComponent Object Reference") (OtherBodyIndex :type Integer) (bFromSweep :type Boolean) (SweepResult :type "HitResult Structure (by ref)")))

(event `self.Sphere.OnComponentHit`
  (params (HitComponent :type "PrimitiveComponent Object Reference") (OtherActor :type "Actor Object Reference") (OtherComp :type "PrimitiveComponent Object Reference") (NormalImpulse :type "Vector Structure") (Hit :type "HitResult Structure (by ref)")))

(event `self.ReceiveTick`
  (params (DeltaSeconds :type "Float (single-precision)"))
  (bind _returnvalue (`self.K2_GetActorLocation`))
  (bind _returnvalue_2 (`self.GetInstigator`))
  (`parent.ReceiveTick` DeltaSeconds)
  (if (`self.bCheck`)
    (bind (_outhit _returnvalue_3) (`KismetSystemLibrary.SphereTraceSingle` (`self.LastLoc`) _returnvalue (`SphereComponent.SphereRadius` (`self.Sphere`)) "TraceTypeQuery4" false (`self.IgnoreList`)))
    (set `self.LastLoc` _returnvalue)
    (if _returnvalue_3
      (bind (_bblockinghit _binitialoverlap _time _distance _location _impactpoint _normal _impactnormal _physmat _hitactor) (`GameplayStatics.BreakHitResult` _outhit))
      (if (not (`KismetArrayLibrary.Array_Contains` (`self.IgnoreList`) _hitactor))
        (bind _asbp_pawn_base (cast `/Game/RL/Core/BP_PawnBase` _hitactor)
          (:`then`
            (if (and (`FGCharacter.IsAlive` _asbp_pawn_base) (`/Game/RL/FunctionLib/FLib_Utility.IsEnemy` _hitactor (`self.GetInstigator`)))
              (if true
                (`|ExecutionSequence` :!label _label
                  (:`then_0`
                    (`AbilitySystemBlueprintLibrary.SendGameplayEventToActor` _returnvalue_2 (struct :`TagName` "Event.Shared.WeaponHit.Bullet") (make `GameplayEventData` (struct :`TagName` "Event.Shared.WeaponHit.Bullet") _returnvalue_2 null (`self.GetOwner`) self (struct) (struct) (struct) 0.0 (`AbilitySystemBlueprintLibrary.AbilityTargetDataFromHitResult` _outhit)))
                    (`KismetSystemLibrary.PrintString` (`KismetStringLibrary.Concat_StrStr` "打中了: " (`KismetSystemLibrary.GetDisplayName` (`.HitActor` (`GameplayStatics.BreakHitResult` _outhit)))) false true (struct :`R` 1.0 :`G` 0.011862 :`A` 1.0))
                    (message `/Game/RL/Interface/BPI_Damage.TakePointDamage` _hitactor 1.0 self (`self.GetInstigator`) _outhit (`self.DamageType`)))
                  (:`then_1`
                    (set `self.bCheck` false :!label _label_2)
                    (`self.OnHit` _outhit)
                    (`self.K2_DestroyActor`))))
              (else
                (goto _label_2))))
          (:`CastFailed`
            (goto _label)))))))

(event `/Game/RL/Interface/BPI_Damage.TakePointDamage`
  (params (Damage :type "Float (single-precision)") (Causer :type "Actor Object Reference") (Instigator :type "Actor Object Reference") (HitResult :type "HitResult Structure") (DamageType :type "DamageType Class Reference"))
  (set `self.bCheck` false)
  (`self.OnHit` HitResult)
  (`self.K2_DestroyActor`))

(fn `GetHitEffects`
  (returns (Sound :type "SoundBase Object Reference") (FX :type "NiagaraSystem Object Reference"))
  (return (`self.HitSound`) (`self.HitFX`)))

(fn `OnHit`
  (params (Hit :type "HitResult Structure (by ref)")))

(fn `TraceForHitResult`
  (returns (OutHit :type "HitResult Structure"))
  (bind _returnvalue (`self.K2_GetActorLocation`))
  (bind _outhit (`KismetSystemLibrary.SphereTraceSingle` :`Start` (+ _returnvalue (* (`self.GetActorForwardVector`) -10.0)) :`End` _returnvalue :`Radius` (`SphereComponent.SphereRadius` (`self.Sphere`)) :`TraceChannel` "TraceTypeQuery1" :`DrawDebugType` "ForDuration"))
  (return _outhit))

(fn `UserConstructionScript`
  (`parent.UserConstructionScript`)
  (`NiagaraComponent.SetAsset` (`self.BodySystem`) (`self.BodyFX`) true))