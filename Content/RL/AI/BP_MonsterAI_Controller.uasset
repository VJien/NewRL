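; AI controller for monsters that runs each monster's behavior tree and mirrors its state into the blackboard.
; Perception picks the first living enemy pawn while no target is valid, passes it to the monster for attack and clears it on death.
; Setters write target, AI stat, locations and distance to blackboard keys, with the Dead stat stopping brain logic.
; SetBlindage claims a blindage as occupant, releasing the previous one.
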(event `self.ReceiveBeginPlay`
  (`KismetSystemLibrary.Delay` 0.2))

(event `self.ReceiveTick`
  (params (DeltaSeconds :type "Float (single-precision)")))

(event `self.AIPerception.OnTargetPerceptionUpdated`
  (params (Actor :type "Actor Object Reference") (Stimulus :type "AIStimulus Structure"))
  (`self.Target`
    (:`then`)
    (:`else`
      (bind _asbp_pawn_base (cast `/Game/RL/Core/BP_PawnBase` Actor))
      (if (`FGCharacter.IsAlive` _asbp_pawn_base)
        (if (`/Game/RL/FunctionLib/FLib_Utility.IsEnemy` (`self.K2_GetPawn`) Actor)
          (`self.SetTarget` Actor)
          (`/Game/RL/AI/BP_MonsterBase.SetAttackTargetActor` (`self.GetControlledMonster`) (`self.Target`))
          (add `/Game/RL/Core/BP_PawnBase.OnDeath` _asbp_pawn_base (delegate `OnTargetDeath`)))))))

(event `OnTargetDeath`
  (params (DeathPawn :type "/Game/RL/Core/BP_PawnBase Object Reference") (SourceASC :type "FGComponent Object Reference") (Damage :type "Float (double-precision)") (`Hit result` :type "HitResult Structure"))
  (`self.SetTarget` null)
  (`/Game/RL/AI/BP_MonsterBase.SetAttackTargetActor` (`self.GetControlledMonster`) null))

(event `self.ReceivePossess`
  (params (PossessedPawn :type "Pawn Object Reference"))
  (`self.RunBehaviorTree` (`/Game/RL/AI/BP_MonsterBase.AI_Behavior` (`self.GetControlledMonster`)))
  (`self.SetInitLocation` (`self.K2_GetActorLocation` PossessedPawn))
  (`self.SetIsAlive` true)
  (`KismetSystemLibrary.Delay` 0.2)
  (bind _asbp_monster_base (cast `/Game/RL/AI/BP_MonsterBase` PossessedPawn))
  (`self.SetAI Stat` (`/Game/RL/AI/BP_MonsterBase.InitializeAI Stat` _asbp_monster_base)))

(fn `GetAttackRange`
  (returns (AttackRange :type "Float (double-precision)"))
  (return (`/Game/RL/AI/BP_MonsterBase.GetAttackRange` (`self.GetControlledMonster`))))

(fn `GetBlindage`
  (returns (Blindage :type "/Game/RL/SceneInstance/BP_AI_Blindage Object Reference"))
  (return (`self.CurrBlindage`)))

(fn `GetControlledMonster`
  (returns (`AsBP Monster Base` :type "/Game/RL/AI/BP_MonsterBase Object Reference"))
  (bind _asbp_monster_base (cast `/Game/RL/AI/BP_MonsterBase` (`self.K2_GetPawn`)))
  (return _asbp_monster_base))

(fn `GetDistanceToTarget`
  (returns (DistanceToTarget :type "Float (double-precision)"))
  (bind _distancetotarget (`self.DistanceToTarget`))
  (if (<= _distancetotarget 0.0)
    (return 9999.0)
    (else
      (return _distancetotarget))))

(fn `GetInitLocation`
  (returns (InitLocation :type "Vector Structure"))
  (return (`self.InitLocation`)))

(fn `GetLastBlindage`
  (returns (Blindage :type "/Game/RL/SceneInstance/BP_AI_Blindage Object Reference"))
  (return (`self.CurrBlindage`)))

(fn `GetTargetActor`
  (returns (Target :type "Actor Object Reference"))
  (return (`self.Target`)))

(fn `SetAI Stat`
  (params (Behavior :type "/Game/RL/Data/Enum/E_AIBehavior Enum" :default "NewEnumerator15"))
  (bind _stat (`self.Stat`))
  (bind _braincomponent (`self.BrainComponent`))
  (bind _returnvalue (`AIBlueprintHelperLibrary.GetBlackboard` self))
  (set `self.Stat` Behavior)
  (`|ExecutionSequence`
    (:`then_0`
      (`/Engine/EditorBlueprintResources/StandardMacros.IsValid` _returnvalue
        (:`Is Valid`
          (`BlackboardComponent.SetValueAsEnum` _returnvalue (`self.Key_Stat`) Behavior))))
    (:`then_1`
      (`self.OnStatChanged` _stat)
      (switch `/Game/RL/Data/Enum/E_AIBehavior` _stat
        (:`NewEnumerator8`
          (`/Engine/EditorBlueprintResources/StandardMacros.IsValid` _braincomponent
            (:`Is Valid`
              (`BrainComponent.StopLogic` _braincomponent ""))))))))

(fn `SetBlindage`
  (params (ObjectValue :type "/Game/RL/SceneInstance/BP_AI_Blindage Object Reference"))
  (`|ExecutionSequence`
    (:`then_0`
      (`/Engine/EditorBlueprintResources/StandardMacros.IsValid` (`self.CurrBlindage`)
        (:`Is Valid`
          (bind _output_get (set `self.LastBlindage` (`self.CurrBlindage`)))
          (`/Game/RL/SceneInstance/BP_AI_Blindage.SetOccupant` _output_get null))))
    (:`then_1`
      (bind _output_get_2 (set `self.CurrBlindage` ObjectValue))
      (`BlackboardComponent.SetValueAsObject` (`AIBlueprintHelperLibrary.GetBlackboard` self) (`self.Key_Blindage`) ObjectValue)
      (`/Engine/EditorBlueprintResources/StandardMacros.IsValid` _output_get_2
        (:`Is Valid`
          (`/Game/RL/SceneInstance/BP_AI_Blindage.SetOccupant` _output_get_2 (`self.GetControlledMonster`)))))))

(fn `SetDestination`
  (params (VectorValue :type "Vector Structure"))
  (`BlackboardComponent.SetValueAsVector` (`AIBlueprintHelperLibrary.GetBlackboard` self) (`self.Key_Destination`) VectorValue))

(fn `SetDistanceToTarget`
  (params (FloatValue :type "Float (double-precision)"))
  (set `self.DistanceToTarget` FloatValue)
  (`BlackboardComponent.SetValueAsFloat` (`AIBlueprintHelperLibrary.GetBlackboard` self) (`self.Key_DistanceToTarget`) FloatValue))

(fn `SetInitLocation`
  (params (VectorValue :type "Vector Structure"))
  (bind _returnvalue (`AIBlueprintHelperLibrary.GetBlackboard` self))
  (`/Engine/EditorBlueprintResources/StandardMacros.IsValid` _returnvalue
    (:`Is Valid`
      (`BlackboardComponent.SetValueAsVector` _returnvalue (`self.Key_InitLocation`) VectorValue)
      (set `self.InitLocation` VectorValue))))

(fn `SetIsAlive`
  (params (BoolValue :type Boolean))
  (`BlackboardComponent.SetValueAsBool` (`AIBlueprintHelperLibrary.GetBlackboard` self) (`self.Key_IsAlive`) BoolValue))

(fn `SetTarget`
  (params (Actor :type "Actor Object Reference"))
  (bind _returnvalue (`AIBlueprintHelperLibrary.GetBlackboard` self))
  (bind _output_get (set `self.Target` Actor))
  (`/Engine/EditorBlueprintResources/StandardMacros.IsValid` _returnvalue
    (:`Is Valid`
      (`BlackboardComponent.SetValueAsObject` _returnvalue (`self.Key_Target`) _output_get))))

(fn `SetTargetIsAlive`
  (params (BoolValue :type Boolean))
  (`BlackboardComponent.SetValueAsBool` (`AIBlueprintHelperLibrary.GetBlackboard` self) (`self.Key_TargetIsAlive`) BoolValue))

(fn `UserConstructionScript`)