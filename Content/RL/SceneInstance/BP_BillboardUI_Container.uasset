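; World-space hint billboard that shows a control-intro widget with configurable text and image, exempted from bullet time.
; Each tick it yaws toward the camera.
; Box overlap with the first valid actor plays a timeline that scales and raises the panel, reversing on exit while a Niagara hint circle toggles.
; DoDestroy plays a sound, hides the panel, then shrinks the icon mesh before destroying the actor.
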(event `self.ReceiveBeginPlay`
  (bind _as_uw_control_intro (`self.As UW Control Intro`))
  (`|ExecutionSequence`
    (:`then_0`
      (bind _asuw_control_intro (cast `/Game/RL/Widget/UW_ControlIntro` (`WidgetComponent.GetWidget` (`self.Widget`))))
      (set `self.As UW Control Intro` _asuw_control_intro)
      (`/Game/RL/Widget/UW_ControlIntro.SetImage` _as_uw_control_intro (`self.Texture`))
      (`/Game/RL/Widget/UW_ControlIntro.SetInfo` _as_uw_control_intro (`self.In Text`)))
    (:`then_1`
      (`/Game/RL/Subsystem/BulletTimeManager/BP_BulletTimeManager.AddIgnoreActor` (subsystem `/Game/RL/Subsystem/BulletTimeManager/BP_BulletTimeManager`) self)
      (set `self.OriginLoc` (`SceneComponent.RelativeLocation` (`self.SM_TextBox_Icon_Info`)))
      (`SceneComponent.SetRelativeScale3D` (`self.ScaleNode`) (0.0 0.0 0.0)))))

(event `self.ReceiveTick`
  (params (DeltaSeconds :type "Float (single-precision)"))
  (`SceneComponent.K2_SetWorldRotation` (`self.Scene`) (`KismetMathLibrary.MakeRotFromXZ` (`KismetMathLibrary.Normal` (- (`PlayerCameraManager.GetCameraLocation` (`GameplayStatics.GetPlayerCameraManager` 0)) (`self.K2_GetActorLocation`))) (`KismetMathLibrary.MakeVector` 0.0 0.0 1.0)) false false))

(event `ShowUI`
  (`ActorComponent.SetActive` (`self.NS_Hint_Circle`) false false)
  (bind (_direction _changerate) (`Timeline|Show` :!label _label)
    (:`Update`
      (`|ExecutionSequence`
        (:`then_0`
          (`SceneComponent.SetRelativeScale3D` (`self.ScaleNode`) (`KismetMathLibrary.Conv_DoubleToVector` _changerate)))
        (:`then_1`
          (`SceneComponent.K2_SetRelativeLocation` (`self.Scene`) (+ (`self.OriginLoc`) (`KismetMathLibrary.MakeVector` 0.0 0.0 (* _changerate 100.0))) false false))))
    (:`Finished`
      (if (`self.Destroy`)
        (bind (_direction_2 _changerate_2) (`Timeline|TimelineDestroy`)
          (:`Update`
            (`SceneComponent.SetRelativeScale3D` (`self.SM_TextBox_Icon_Info`) (`KismetMathLibrary.Conv_DoubleToVector` _changerate_2)))
          (:`Finished`
            (`self.K2_DestroyActor`)))))))

(event `HideUI`
  (bind _returnvalue (not (`self.Destroy`)))
  (`ActorComponent.SetActive` (`self.NS_Hint_Circle`) _returnvalue _returnvalue)
  (goto _label :!via `Reverse`))

(event `DoDestroy`
  (if (not (`self.Destroy`))
    (set `self.Destroy` true)
    (`self.HideUI`)
    (`GameplayStatics.PlaySound2D` "/Game/RL/Sound/UI/Sure.Sure" 1.0 1.0 0.0 null null)))

(event `self.Box.OnComponentBeginOverlap`
  (params (OverlappedComponent :type "PrimitiveComponent Object Reference") (OtherActor :type "Actor Object Reference") (OtherComp :type "PrimitiveComponent Object Reference") (OtherBodyIndex :type Integer) (bFromSweep :type Boolean) (SweepResult :type "HitResult Structure (by ref)"))
  ;[1 1 1] Trigger
  (`/Engine/EditorBlueprintResources/StandardMacros.IsValid` (`self.Overlap Actor`)
    (:`Is Not Valid`
      (set `self.Overlap Actor` OtherActor)
      (`self.ShowUI`))))

(event `self.Box.OnComponentEndOverlap`
  (params (OverlappedComponent :type "PrimitiveComponent Object Reference") (OtherActor :type "Actor Object Reference") (OtherComp :type "PrimitiveComponent Object Reference") (OtherBodyIndex :type Integer))
  ;[1 1 1] Trigger
  (if (== OtherActor (`self.Overlap Actor`))
    (`self.HideUI`)
    (set `self.Overlap Actor` null)))

(event `SetTextInfo`
  (params (InText :type Text))
  (bind _as_uw_control_intro (`self.As UW Control Intro`))
  ;[1 1 1] SetUI
  (`/Engine/EditorBlueprintResources/StandardMacros.IsValid` _as_uw_control_intro
    (:`Is Valid`
      (bind _output_get (set `self.In Text` InText))
      (`/Game/RL/Widget/UW_ControlIntro.SetInfo` _as_uw_control_intro _output_get))))

(event `SetImage`
  (params (Texture :type "Texture2D Object Reference"))
  (bind _as_uw_control_intro (`self.As UW Control Intro`))
  ;[1 1 1] SetUI
  (`/Engine/EditorBlueprintResources/StandardMacros.IsValid` _as_uw_control_intro
    (:`Is Valid`
      (bind _output_get (set `self.Texture` Texture))
      (`/Game/RL/Widget/UW_ControlIntro.SetImage` _as_uw_control_intro _output_get))))

(fn `UserConstructionScript`
  (`BoxComponent.SetBoxExtent` (`self.Box`) (`self.Box Extent`) true))