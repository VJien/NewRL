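; Bullet-time manager that drives global time dilation in power or infinite mode.
; Power mode switches between Enter, EnterMove and Jump states, draining a meter that refills after a delay in real time.
; Infinite mode maps head and hand movement speed through a curve to time scale.
; Wall-clock milliseconds supply undilated delta time, and ignored or specified actors get compensating CustomTimeDilation whenever the scale changes.
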(event `self.OnInit`
  (bind (_returnvalue_year _returnvalue_month _returnvalue_day _returnvalue_hour _returnvalue_minute _returnvalue_second _returnvalue_millisecond) (`KismetMathLibrary.BreakDateTime` (`KismetMathLibrary.Now`)))
  (`|ExecutionSequence`
    (:`then_0`
      (set `self.CurrentStatus` "NewEnumerator0")
      (set `self.IsInPowerModeBulletTime` false)
      (set `self.PowerPercent` 1.0)
      (set `self.RecoverCount` 0.0))
    (:`then_1`
      (set `self.RealTimeDuration` -1.0))
    (:`then_2`
      (set `self.TimeRate` 1.0)
      (set `self.Infinite` false)
      (set `self.LastMillisecond` _returnvalue_millisecond))))

(event `self.OnTick`
  (params (DeltaTime :type "Float (single-precision)"))
  (bind (_returnvalue_year _returnvalue_month _returnvalue_day _returnvalue_hour _returnvalue_minute _returnvalue_second _returnvalue_millisecond) (`KismetMathLibrary.BreakDateTime` (`KismetMathLibrary.Now`)))
  (bind (_config_powerrecoverstatictime _config_recoverpowerrate) (break `/Game/RL/Subsystem/BulletTimeManager/SBulletTimeConfig` (`self.Config`)))
  (`|ExecutionSequence`
    (:`then_0`
      (if (`self.IsUpdateCustomActors`)
        (`self.SetCustomActorsTimeScale`)
        (set `self.IsUpdateCustomActors` false)))
    (:`then_1`
      (set `self.CurDeltaTime` (/ (`KismetMathLibrary.Conv_IntToDouble` (mod (- (+ _returnvalue_millisecond 1000) (`self.LastMillisecond`)) 1000)) 1000.0))
      (set `self.LastMillisecond` _returnvalue_millisecond))
    (:`then_2`
      (if (`self.Infinite`)
        (`self.CheckInfiniteTimeScale` (`self.CurDeltaTime`))
        (else
          ;[1 1 1] PowerMode
          (if (`self.IsInPowerModeBulletTime`)
            (bind _output_get (set `self.PowerPercent` (- (`self.PowerPercent`) (`self.GetConsumeByTime` (`self.CurDeltaTime`)))))
            (if (> _output_get 0.0)
              (`self.CheckPowerModeTimeScale` (`self.CurDeltaTime`))
              (else
                (set `self.PowerPercent` 0.0)
                (`self.ChangeBulletTime` "NewEnumerator0")))
            (elif (>= (`self.RecoverCount`) _config_powerrecoverstatictime)
              (set `self.PowerPercent` (`KismetMathLibrary.FClamp` (+ (`self.PowerPercent`) (* DeltaTime _config_recoverpowerrate))))
              (else
                (set `self.RecoverCount` (+ (`self.RecoverCount`) DeltaTime))))))))))

(event `RegisterMoveNode`
  (params (Head :type "SceneComponent Object Reference") (Hand :type "Array of SceneComponent Object Reference"))
  (`KismetArrayLibrary.Array_Clear` (`self.MoveNodeInfo`))
  (`|ExecutionSequence`
    (:`then_0`
      (`/Engine/EditorBlueprintResources/StandardMacros.IsValid` Head
        (:`Is Valid`
          (`KismetArrayLibrary.Array_Add` (`self.MoveNodeInfo`) (make `/Game/RL/Subsystem/BulletTimeManager/SBulletTimeMoveNodeInfo` Head (`SceneComponent.K2_GetComponentLocation` Head))))))
    (:`then_1`
      (for _array_element Hand
        (`KismetArrayLibrary.Array_Add` (`self.MoveNodeInfo`) (make `/Game/RL/Subsystem/BulletTimeManager/SBulletTimeMoveNodeInfo` _array_element (`SceneComponent.K2_GetComponentLocation` _array_element)))))))

(event `ChangeMode`
  (params (Infinite :type Boolean))
  (bind _movenodeinfo (`self.MoveNodeInfo`))
  (bind _output_get (set `self.Infinite` (and Infinite (> (`KismetArrayLibrary.Array_Length` (`self.MoveNodeInfo`)) 0))))
  (if _output_get
    (set `self.RealTimeDuration` -1.0)
    (`self.SetTimeScale` 0.0)
    (for (_array_element _array_index) _movenodeinfo
      (setmembers `/Game/RL/Subsystem/BulletTimeManager/SBulletTimeMoveNodeInfo` :`StructRef` (`|GetArrayItem` _movenodeinfo _array_index) :`LastPos` (`SceneComponent.K2_GetComponentLocation` (`.MoveNode_2_97E29645458C69FC62F6B5BE4E7D3781` (break `/Game/RL/Subsystem/BulletTimeManager/SBulletTimeMoveNodeInfo` _array_element)))))
    (else
      (set `self.CurrentStatus` "NewEnumerator0")
      (`self.SetTimeScale` 1.0))))

(event `EnterRealTimeWithTime(Infinite)`
  (params (Duration :type "Float (double-precision)" :default 1.0))
  ;[1 1 1] Infinite
  (set `self.RealTimeDuration` Duration)
  (if (`self.Infinite`)
    (`self.SetTimeScale` 1.0)))

(event `EnterPowerModeBulletTime`
  (params (IsJump :type Boolean))
  ;[1 1 1] PowerMode
  (if IsJump
    (`self.ChangeBulletTime` "NewEnumerator3")
    (else
      (`self.ChangeBulletTime` "NewEnumerator1"))))

(event `QuitPowerModeBulletTime`
  ;[1 1 1] PowerMode
  (`self.ChangeBulletTime` "NewEnumerator0"))

(fn `AddIgnoreActor`
  (params (Aim :type "Actor Object Reference"))
  (`|ExecutionSequence`
    (:`then_0`
      (set `Actor.CustomTimeDilation` (/ 1.0 (`self.TimeRate`)) Aim))
    (:`then_1`
      (`KismetArrayLibrary.Array_AddUnique` (`self.IgnoreActor`) Aim))))

(fn `AddSpecifyActor`
  (params (Actor :type "Actor Object Reference") (SpecifyTimeRate :type "Float (double-precision)" :default 1.0))
  (bind _specifyactorlist (`self.SpecifyActorList`))
  (`/Engine/EditorBlueprintResources/StandardMacros.IsValid` Actor
    (:`Is Valid`
      (if (not (`.ReturnValue` (`BlueprintMapLibrary.Map_Find` _specifyactorlist Actor)))
        (`BlueprintMapLibrary.Map_Add` _specifyactorlist Actor (`KismetMathLibrary.FClamp` SpecifyTimeRate))))))

(fn `ChangeBulletTime`
  (params (AimStatus :type "/Game/RL/Subsystem/BulletTimeManager/EBulletTimeStatus Enum" :default "NewEnumerator0"))
  (bind _movenodeinfo (`self.MoveNodeInfo`))
  (bind _currentstatus (`self.CurrentStatus`))
  (bind _currentstatus_2 (`self.CurrentStatus`))
  (bind ((`RecoverPowerRate_24_FFBE2D314878DE2D67F30FA5A5C57FAC` _recoverpowerrate) (`MoveProtectMaxSpeed_29_EBC919904D9F6509D3A691A2E1C98577` _moveprotectmaxspeed) (`RealTimeRateConsume_36_5161555E431CCE0F594982AC57203DE3` _realtimerateconsume) (`EnterRateConsume_38_AB5CC2EB4D13BA21D99D139F569DB45D` _enterrateconsume) (`EnterMoveRateConsume_42_6D6BCF684C674418DA6F0C85D2ED3099` _entermoverateconsume) (`JumpRateConsume_44_996B4A724DFB66F56F0785AB7C9213D3` _jumprateconsume)) (break `/Game/RL/Subsystem/BulletTimeManager/SBulletTimeConfig` (`self.Config`)))
  (bind _returnvalue (> (`self.PowerPercent`) 0.0))
  (bind _returnvalue_2 (> (`self.PowerPercent`) 0.0))
  ;[1 1 1] if need manager status
  (switch `/Game/RL/Subsystem/BulletTimeManager/EBulletTimeStatus` AimStatus
    (:`NewEnumerator0`
      (if (`|EnumInequality` (`self.CurrentStatus`) "NewEnumerator0")
        (set `self.IsInPowerModeBulletTime` false)
        (set `self.RecoverCount` 0.0)
        (`|ExecutionSequence`
          (:`then_0`
            (bind _output_get (set `self.CurrentStatus` AimStatus :!label _label))
            (`self.SetTimeScale` (select `/Game/RL/Subsystem/BulletTimeManager/EBulletTimeStatus` _output_get :`NewEnumerator0` (`KismetMathLibrary.BreakVector2D` _realtimerateconsume) :`NewEnumerator1` (`KismetMathLibrary.BreakVector2D` _enterrateconsume) :`NewEnumerator2` (`KismetMathLibrary.BreakVector2D` _entermoverateconsume) :`NewEnumerator3` (`KismetMathLibrary.BreakVector2D` _jumprateconsume))))
          (:`then_1`
            (`self.BulletTimeStopHandler`)))
        (else
          (return))))
    (:`NewEnumerator1`
      (if (and (`|EnumEquality` (`self.CurrentStatus`) "NewEnumerator0") _returnvalue)
        (set `self.IsInPowerModeBulletTime` true)
        (`|ExecutionSequence`
          (:`then_0`
            (goto _label))
          (:`then_1`
            (`self.BulletTimeStartHandler` "NewEnumerator1"))
          (:`then_2`
            (for (_array_element _array_index) _movenodeinfo
              (setmembers `/Game/RL/Subsystem/BulletTimeManager/SBulletTimeMoveNodeInfo` :`StructRef` (`|GetArrayItem` _movenodeinfo _array_index) :`LastPos` (`SceneComponent.K2_GetComponentLocation` (`.MoveNode_2_97E29645458C69FC62F6B5BE4E7D3781` (break `/Game/RL/Subsystem/BulletTimeManager/SBulletTimeMoveNodeInfo` _array_element)))))))
        (elif (and _returnvalue (or (`|EnumEquality` _currentstatus_2 "NewEnumerator2") (`|EnumEquality` _currentstatus_2 "NewEnumerator3")))
          (`|ExecutionSequence`
            (:`then_0`
              (goto _label))
            (:`then_1`
              (`self.BulletTimeStatusChangeHandler` "NewEnumerator1")))
          (else
            (return)))))
    (:`NewEnumerator2`
      (if (`|EnumEquality` (`self.CurrentStatus`) "NewEnumerator1")
        (`|ExecutionSequence`
          (:`then_0`
            (goto _label))
          (:`then_1`
            (`self.BulletTimeStatusChangeHandler` "NewEnumerator2")))
        (else
          (return))))
    (:`NewEnumerator3`
      (if (and (`|EnumEquality` (`self.CurrentStatus`) "NewEnumerator0") _returnvalue_2)
        (set `self.IsInPowerModeBulletTime` true)
        (`|ExecutionSequence`
          (:`then_0`
            (goto _label))
          (:`then_1`
            (`self.BulletTimeStartHandler` "NewEnumerator3")))
        (elif (and _returnvalue_2 (or (`|EnumEquality` _currentstatus "NewEnumerator2") (`|EnumEquality` _currentstatus "NewEnumerator1")))
          (`|ExecutionSequence`
            (:`then_0`
              (goto _label))
            (:`then_1`
              (`self.BulletTimeStatusChangeHandler` "NewEnumerator3")))
          (else
            (return)))))))

(fn `CheckInfiniteTimeScale`
  (params (DeltaTime :type "Float (double-precision)"))
  (locals (MaxTimeScale :type "Float (double-precision)" :default 0.0))
  (bind _movenodeinfo (`self.MoveNodeInfo`))
  (`|ExecutionSequence`
    (:`then_0`
      (set `local.MaxTimeScale` 0.0))
    (:`then_1`
      (for (_array_element _array_index) _movenodeinfo
        (`|ExecutionSequence`
          (:`then_0`
            (bind (_movenode _lastpos _smoothlocspeedrange) (break `/Game/RL/Subsystem/BulletTimeManager/SBulletTimeMoveNodeInfo` _array_element))
            (bind _returnvalue (`SceneComponent.K2_GetComponentLocation` _movenode))
            (bind (_x _y) (`KismetMathLibrary.BreakVector2D` _smoothlocspeedrange))
            (set `local.MaxTimeScale` (`KismetMathLibrary.FMax` (`local.MaxTimeScale`) (/ (- (/ (`KismetMathLibrary.Vector_Distance` _returnvalue _lastpos) DeltaTime) _x) (- _y _x)))))
          (:`then_1`
            (setmembers `/Game/RL/Subsystem/BulletTimeManager/SBulletTimeMoveNodeInfo` :`StructRef` (`|GetArrayItem` _movenodeinfo _array_index) :`LastPos` _returnvalue)))))
    (:`then_2`
      (if (> (`self.RealTimeDuration`) 0.0)
        (set `self.RealTimeDuration` (- (`self.RealTimeDuration`) DeltaTime))
        (else
          (`self.SetTimeScale` (`CurveFloat.GetFloatValue` (`self.CB_InfiniteTimeScale`) (`local.MaxTimeScale`))))))))

(fn `CheckPowerModeTimeScale`
  (params (DeltaTime :type "Float (double-precision)"))
  (locals (MaxMoveSpeed :type "Float (double-precision)" :default 0.0))
  (bind _movenodeinfo (`self.MoveNodeInfo`))
  (`|ExecutionSequence`
    (:`then_0`
      (set `local.MaxMoveSpeed` 0.0))
    (:`then_1`
      (for (_array_element _array_index) _movenodeinfo
        (`|ExecutionSequence`
          (:`then_0`
            (bind (_movenode _lastpos) (break `/Game/RL/Subsystem/BulletTimeManager/SBulletTimeMoveNodeInfo` _array_element))
            (bind _returnvalue (`SceneComponent.K2_GetComponentLocation` _movenode))
            (set `local.MaxMoveSpeed` (`KismetMathLibrary.FMax` (`local.MaxMoveSpeed`) (`KismetMathLibrary.FMax` (- (/ (`KismetMathLibrary.Vector_Distance` _returnvalue _lastpos) DeltaTime) (`.MoveProtectMaxSpeed_29_EBC919904D9F6509D3A691A2E1C98577` (break `/Game/RL/Subsystem/BulletTimeManager/SBulletTimeConfig` (`self.Config`))))))))
          (:`then_1`
            (setmembers `/Game/RL/Subsystem/BulletTimeManager/SBulletTimeMoveNodeInfo` :`StructRef` (`|GetArrayItem` _movenodeinfo _array_index) :`LastPos` _returnvalue)))))
    (:`then_2`
      (if (`|EnumInequality` (`self.CurrentStatus`) "NewEnumerator3")
        (if (> (`local.MaxMoveSpeed`) 0.0)
          (`self.ChangeBulletTime` "NewEnumerator2")
          (else
            (`self.ChangeBulletTime` "NewEnumerator1")))))))

(fn `GetConsumeByTime`
  (params (RealTimeDelta :type "Float (double-precision)"))
  (returns (ReturnValue :type "Float (double-precision)"))
  (bind ((`RealTimeRateConsume_36_5161555E431CCE0F594982AC57203DE3` _realtimerateconsume) (`EnterRateConsume_38_AB5CC2EB4D13BA21D99D139F569DB45D` _enterrateconsume) (`EnterMoveRateConsume_42_6D6BCF684C674418DA6F0C85D2ED3099` _entermoverateconsume) (`JumpRateConsume_44_996B4A724DFB66F56F0785AB7C9213D3` _jumprateconsume)) (break `/Game/RL/Subsystem/BulletTimeManager/SBulletTimeConfig` (`self.Config`)))
  (return (* RealTimeDelta (select `/Game/RL/Subsystem/BulletTimeManager/EBulletTimeStatus` (`self.CurrentStatus`) :`NewEnumerator0` (`.Y` (`KismetMathLibrary.BreakVector2D` _realtimerateconsume)) :`NewEnumerator1` (`.Y` (`KismetMathLibrary.BreakVector2D` _enterrateconsume)) :`NewEnumerator2` (`.Y` (`KismetMathLibrary.BreakVector2D` _entermoverateconsume)) :`NewEnumerator3` (`.Y` (`KismetMathLibrary.BreakVector2D` _jumprateconsume))))))

(fn `GetCurrentPowerPercent`
  (returns (Power :type "Float (double-precision)"))
  (return (`self.PowerPercent`)))

(fn `GetMaxJumpTime`
  (returns (Seconds :type "Float (double-precision)"))
  (return (/ (`self.PowerPercent`) (`.Y` (`KismetMathLibrary.BreakVector2D` (`.JumpRateConsume_44_996B4A724DFB66F56F0785AB7C9213D3` (break `/Game/RL/Subsystem/BulletTimeManager/SBulletTimeConfig` (`self.Config`))))))))

(fn `IsInBulletTime`
  (params (ItemToFind :type "Actor Object Reference (by ref)"))
  (returns (ReturnValue :type Boolean))
  (bind _ignoreactor (`self.IgnoreActor`))
  (`/Engine/EditorBlueprintResources/StandardMacros.IsValid` ItemToFind
    (:`Is Valid`
      (if (`KismetArrayLibrary.Array_IsValidIndex` _ignoreactor (`KismetArrayLibrary.Array_Find` _ignoreactor ItemToFind))
        (return false)
        (else
          _)))
    (:`Is Not Valid`
      _))
  (return (or (`self.IsInPowerModeBulletTime`) (`self.Infinite`))))

(fn `RemoveIgnoreActor`
  (params (Item :type "Actor Object Reference (by ref)"))
  (bind _returnvalue (`KismetArrayLibrary.Array_RemoveItem` (`self.IgnoreActor`) Item))
  (if _returnvalue
    (set `Actor.CustomTimeDilation` 1.0 Item)))

(fn `RemoveSpecifyActor`
  (params (Actor :type "Actor Object Reference (by ref)"))
  (bind _returnvalue (`BlueprintMapLibrary.Map_Remove` (`self.SpecifyActorList`) Actor))
  (if _returnvalue
    (set `Actor.CustomTimeDilation` 1.0 Actor)))

(fn `SetCustomActorsTimeScale`
  (locals (Count :type Integer))
  (bind _output (`|GetArrayItem` (`self.IgnoreActor`) (`local.Count`)))
  (`|ExecutionSequence`
    (:`then_0`
      ;[1 1 1] SpecifyActorCheck
      (set `local.Count` 0)
      (if (< (`local.Count`) (`BlueprintMapLibrary.Map_Length` (`self.SpecifyActorList`))) :!label _label
        (bind _keys (`BlueprintMapLibrary.Map_Keys` (`self.SpecifyActorList`)))
        (bind _output_2 (`|GetArrayItem` _keys (`local.Count`)))
        (`/Engine/EditorBlueprintResources/StandardMacros.IsValid` _output_2
          (:`Is Valid`
            (set `Actor.CustomTimeDilation` (/ (select `bool` (or (`self.Infinite`) (`self.IsInPowerModeBulletTime`)) :`false` 1.0 :`true` (`BlueprintMapLibrary.Map_Find` (`self.SpecifyActorList`) _output_2)) (`self.TimeRate`)) _output_2)
            (`/Engine/EditorBlueprintResources/StandardMacros.IncrementInt` (`local.Count`)
              (:`  `
                (goto _label))))
          (:`Is Not Valid`
            (`BlueprintMapLibrary.Map_Remove` (`self.SpecifyActorList`) _output_2)
            (goto _label)))))
    (:`then_1`
      ;[1 1 1] Ignore  Actor  Check
      (set `local.Count` 0)
      (if (< (`local.Count`) (`KismetArrayLibrary.Array_Length` (`self.IgnoreActor`))) :!label _label_2
        (`/Engine/EditorBlueprintResources/StandardMacros.IsValid` _output
          (:`Is Valid`
            (set `Actor.CustomTimeDilation` (/ 1.0 (`self.TimeRate`)) _output)
            (`/Engine/EditorBlueprintResources/StandardMacros.IncrementInt` (`local.Count`)
              (:`  `
                (goto _label_2))))
          (:`Is Not Valid`
            (`KismetArrayLibrary.Array_Remove` (`self.IgnoreActor`) (`local.Count`))
            (goto _label_2)))))))

(fn `SetTimeScale`
  (params (Scale :type "Float (double-precision)"))
  (`|ExecutionSequence`
    (:`then_0`
      (set `self.TimeRate` (`KismetMathLibrary.FClamp` Scale 0.001))
      (`GameplayStatics.SetGlobalTimeDilation` (`self.TimeRate`)))
    (:`then_1`
      (set `self.IsUpdateCustomActors` true))))

(fn `TransGameTimeToRealTime`
  (params (GameTime :type "Float (double-precision)"))
  (returns (ReturnValue :type "Float (double-precision)"))
  (return (/ GameTime (`self.TimeRate`))))

(fn `TransRealTimeToGameTime`
  (params (RealTime :type "Float (double-precision)"))
  (returns (ReturnValue :type "Float (double-precision)"))
  (return (* RealTime (`self.TimeRate`))))