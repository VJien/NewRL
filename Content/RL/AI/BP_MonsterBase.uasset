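; Base AI monster character for a VR shooter, with a child-actor weapon, camera-facing health bar, montage reactions and random sounds.
; Its AI stat is pushed to BP_MonsterAI_Controller, whose change event sets movement speed and rotation.
; Attacks play a montage and fire the weapon with randomised aim; damage without a target reports sense events.
; It registers with BP_AI_Blindage cover points, line-tracing for sight of the target, and supports ragdoll death.
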(event `self.PostDamage`
  (params (SourceASC :type "FGComponent Object Reference") (Damage :type "Float (single-precision)") (HitResult :type "HitResult Structure"))
  (bind (_actorinfo _returnvalue) (`FGBlueprintLibrary.TryGetActorInfo` SourceASC))
  (bind _returnvalue_2 (`self.K2_GetActorLocation`))
  (bind ((`AvatarActor` _avataractor)) (break `GameplayAbilityActorInfo` _actorinfo))
  (bind _outitem (`KismetArrayLibrary.Array_Random` (`self.HurtAnimMontages`)))
  (`KismetSystemLibrary.PrintString` (`FGBlueprintLibrary.UStructToJsonObjectString` (`FGBlueprintLibrary.TryGetActorInfo` SourceASC)) false)
  (if (`FGCharacter.IsAlive`)
    (`|ExecutionSequence`
      (:`then_0`
        (`self.SetAI Stat` "NewEnumerator14")
        (if (`self.bShouldPlayHurtAnimation`)
          (`/Engine/EditorBlueprintResources/StandardMacros.IsValid` _outitem
            (:`Is Valid`
              (`|PlayMontage` (`self.Mesh`) _outitem
                (:`OnCompleted`
                  (`self.SetAI Stat` "NewEnumerator15" :!label _label))
                (:`OnInterrupted`
                  (`KismetSystemLibrary.PrintString` "*****受伤被打断!" false))))
            (:`Is Not Valid`
              (goto _label)))
          (else
            (`self.SetAI Stat` "NewEnumerator15"))))
      (:`then_1`
        (`/Engine/EditorBlueprintResources/StandardMacros.IsValid` (`self.GetAttackTargetActor`)
          (:`Is Not Valid`
            (if _returnvalue
              (if (`self.bReportEventWhenDamaged`)
                (`AISense_Damage.ReportDamageEvent` self _avataractor 1.0 _returnvalue_2 _returnvalue_2)
                (`AISense_Hearing.ReportNoiseEvent` _returnvalue_2 1.0 _avataractor 2000.0)))))))))

(event `PlayAttackAnimation`
  (`|PlayMontage` (`self.Mesh`) (`KismetArrayLibrary.Array_Random` (`self.AttackAnimation`))
    (:`OnCompleted`
      _)
    (:`OnInterrupted`
      _))
  (`self.FinishAttack`))

(event `self.ReceiveBeginPlay`
  (`|ExecutionSequence`
    (:`then_0`
      (bind _asbpi_interactable_item (cast `/Game/RL/Interface/BPI_InteractableItem` (`ChildActorComponent.ChildActor` (`self.WeaponChildActor`))))
      (`/Game/RL/Interface/BPI_InteractableItem.TargetBeGrab` _asbpi_interactable_item self self "NewEnumerator7"))
    (:`then_1`
      (bind _asuw_monster_stat_bar (cast `/Game/RL/Widget/UW_MonsterStatBar` (`WidgetComponent.GetUserWidgetObject` (`self.Widget`))))
      (`/Game/RL/Widget/UW_MonsterStatBar.Init` _asuw_monster_stat_bar self))
    (:`then_3`
      (`self.PlayStartSound`)
      (`self.SetMoveSpeed` (`self.InitSpeed`)))))

(event `self.ReceiveTick`
  (params (DeltaSeconds :type "Float (single-precision)"))
  (bind _widget (`self.Widget`))
  (bind (_returnvalue_roll _returnvalue_pitch _returnvalue_yaw) (`KismetMathLibrary.BreakRotator` (`KismetMathLibrary.FindLookAtRotation` (`SceneComponent.K2_GetComponentLocation` _widget) (`PlayerCameraManager.GetCameraLocation` (`GameplayStatics.GetPlayerCameraManager` 0)))))
  (`SceneComponent.K2_SetWorldRotation` _widget (`KismetMathLibrary.MakeRotator` 0.0 0.0 _returnvalue_yaw) false false))

(event `self.ReceivePossessed`
  (params (NewController :type "Controller Object Reference"))
  (bind _asbp_monster_ai_controller (cast `/Game/RL/AI/BP_MonsterAI_Controller` NewController))
  (add `/Game/RL/AI/BP_MonsterAI_Controller.OnStatChanged` _asbp_monster_ai_controller (`|CreateDelegate` :!event `OnStatChanged`))
  (`self.SetAI Stat` (`self.InitializeAI Stat`))
  (bind _outactors (`GameplayStatics.GetAllActorsOfClass` "/Game/RL/SceneInstance/BP_AI_Blindage.BP_AI_Blindage_C"))
  (bind _output_get (set `self.Blindages` _outactors))
  (`KismetSystemLibrary.Delay` 0.2)
  (for _array_element _output_get
    (`/Game/RL/SceneInstance/BP_AI_Blindage.RegisterMonster` _array_element self)))

(fn `DoAttack`
  (params (Event :type "Delegate (by ref)"))
  (locals (Target :type "Vector Structure" :default (0.0 0.0 0.0)))
  (bind _asbp_weapon_base (`self.GetGun`))
  (bind _attacktargetactor (`self.GetAttackTargetActor`))
  (add `self.OnAttackFinish` Event)
  (`self.PlayAttackAnimation`)
  (`MovementComponent.StopMovementImmediately` (`self.CharacterMovement`))
  (`/Engine/EditorBlueprintResources/StandardMacros.IsValid` _asbp_weapon_base
    (:`Is Valid`
      (`|ExecutionSequence`
        (:`then_0`
          (`/Engine/EditorBlueprintResources/StandardMacros.IsValid` _attacktargetactor
            (:`Is Valid`
              (bind _asbp_vr_pawn (cast `/Game/RL/Core/BP_VR_Pawn` _attacktargetactor)
                (:`then`
                  (set `local.Target` (`self.GetAimTargetPostion` _asbp_vr_pawn)))
                (:`CastFailed`
                  (set `local.Target` (`self.K2_GetActorLocation` _attacktargetactor)))))))
        (:`then_1`
          (`/Game/RL/Core/BP_ItemBase.TryUseItem` _asbp_weapon_base self self))))))

(fn `DoDeath`
  (params (SourceASC :type "FGComponent Object Reference") (Damage :type "Float (double-precision)") (HitResult :type "HitResult Structure"))
  (bind _asabp_monster (`self.GetMonsterAnimInstance`))
  (`KismetSystemLibrary.PrintString` "*****死亡*****" false)
  (`AnimInstance.Montage_Stop` _asabp_monster 0.0 (`AnimInstance.GetCurrentActiveMontage` _asabp_monster))
  (`self.SetAI Stat` "NewEnumerator8")
  (`self.PlayAnimMontage` (`KismetArrayLibrary.Array_Random` (`self.DeadAnimMontages`)))
  (`SceneComponent.SetHiddenInGame` (`self.Widget`) true false)
  (`MovementComponent.StopMovementImmediately` (`self.CharacterMovement`))
  (`self.SetLifeSpan` 5.0)
  (`self.PlayDeadSound`)
  (`SceneComponent.SetVisibility` (`self.WeaponChildActor`) false false))

(fn `DoPhysicsDeath`
  (params (Hit :type "HitResult Structure"))
  (bind (_bblockinghit _binitialoverlap _time _distance _location _impactpoint _normal _impactnormal _physmat _hitactor _hitcomponent _hitbonename) (`GameplayStatics.BreakHitResult` Hit))
  (bind _mesh (`self.Mesh`))
  (if (`self.bUseRagdollDeath`)
    (`PrimitiveComponent.SetCollisionProfileName` _mesh "Ragdoll" true)
    (`PrimitiveComponent.SetSimulatePhysics` _mesh true)
    (`PrimitiveComponent.AddImpulseAtLocation` (`self.Mesh`) (* (* _impactnormal -1.0) 10000.0) _impactpoint _hitbonename)
    (else
      (`PrimitiveComponent.SetCollisionEnabled` (`self.Mesh`) "NoCollision"))))

(fn `FinishAttack`
  (`self.OnAttackFinish`))

(fn `GetAttackRange`
  (returns (AttackRange :type "Float (double-precision)"))
  (return (`self.AttackRange`)))

(fn `GetAttackTargetActor`
  (returns (AttackTargetActor :type "Actor Object Reference"))
  (return (`self.AttackTargetActor`)))

(fn `GetCurrentWeapon`
  (params (Hand :type "/Game/RL/Data/Enum/E_HandType Enum" :default "NewEnumerator7"))
  (returns (Weapon :type "/Game/RL/Weapon/BP_WeaponBase Object Reference"))
  (bind _asbp_weapon_base (cast `/Game/RL/Weapon/BP_WeaponBase` (`ChildActorComponent.ChildActor` (`self.WeaponChildActor`))))
  (return _asbp_weapon_base))

(fn `GetGun`
  (returns (`AsBP Weapon Base` :type "/Game/RL/Weapon/BP_WeaponBase Object Reference"))
  (bind _asbp_weapon_base (cast `/Game/RL/Weapon/BP_WeaponBase` (`ChildActorComponent.ChildActor` (`self.WeaponChildActor`))))
  (return _asbp_weapon_base))

(fn `GetHurtAnimMontage`
  (returns (Montage :type "AnimMontage Object Reference"))
  (return (`KismetArrayLibrary.Array_Random` (`self.HurtAnimMontages`))))

(fn `GetInitSpeed`
  (returns (InitSpeed :type "Float (double-precision)"))
  (return (`self.InitSpeed`)))

(fn `GetMonsterAnimInstance`
  (returns (`AsABP Monster` :type "/Game/RL/AI/Animation/ABP_Monster Object Reference"))
  (bind _asabp_monster (cast `/Game/RL/AI/Animation/ABP_Monster` (`SkeletalMeshComponent.GetAnimInstance` (`self.Mesh`))))
  (return _asabp_monster))

(fn `GetMonsterFirePosition`
  (returns (ReturnValue :type "Transform Structure"))
  (locals (randomCameraLoc :type "Vector Structure" :default (0.0 0.0 0.0)) (AimOffset :type "Float (double-precision)" :default 20.0))
  (bind _attacktargetactor (`self.GetAttackTargetActor`))
  (bind _aimoffset (`local.AimOffset`))
  (bind _aimoffset_2 (`local.AimOffset`))
  (bind _aimoffset_3 (`local.AimOffset`))
  (bind _returnvalue (`SceneComponent.GetSocketTransform` (`self.Mesh`) (`self.Socket_Shoot`) "RTS_World"))
  (bind _location (.location _returnvalue))
  (`/Engine/EditorBlueprintResources/StandardMacros.IsValid` _attacktargetactor
    (:`Is Valid`
      (bind _asbp_vr_pawn (cast `/Game/RL/Core/BP_VR_Pawn` _attacktargetactor)
        (:`then`
          (bind _output_get (set `local.randomCameraLoc` (+ (`SceneComponent.K2_GetComponentLocation` (`/Game/RL/Core/BP_VR_Pawn.Camera` _asbp_vr_pawn)) (`KismetMathLibrary.MakeVector` (`KismetMathLibrary.RandomFloatInRange` (* _aimoffset_2 -1.0) _aimoffset_2) (`KismetMathLibrary.RandomFloatInRange` (* _aimoffset_3 -1.0) _aimoffset_3) (`KismetMathLibrary.RandomFloatInRange` (* _aimoffset -1.0) _aimoffset)))))
          (return (`KismetMathLibrary.MakeTransform` _location (`KismetMathLibrary.FindLookAtRotation` _location _output_get))))
        (:`CastFailed`
          (return (`KismetMathLibrary.MakeTransform` _location (`KismetMathLibrary.FindLookAtRotation` _location (+ (`self.K2_GetActorLocation` _attacktargetactor) (`KismetMathLibrary.MakeVector` (`KismetMathLibrary.RandomFloatInRange` -20.0 20.0) (`KismetMathLibrary.RandomFloatInRange` -20.0 20.0) (`KismetMathLibrary.RandomFloatInRange` -20.0 20.0)) (0.0 0.0 40.0))))))))
    (:`Is Not Valid`
      (return _returnvalue))))

(fn `Is Blindage in Weapon View`
  (params (NewParam :type "/Game/RL/SceneInstance/BP_AI_Blindage Object Reference"))
  (returns (ReturnValue :type Boolean))
  (locals (TargetLocation :type "Vector Structure"))
  (bind _attacktargetactor (`self.GetAttackTargetActor`))
  (`/Engine/EditorBlueprintResources/StandardMacros.IsValid` NewParam
    (:`Is Valid`
      (`/Engine/EditorBlueprintResources/StandardMacros.IsValid` _attacktargetactor
        (:`Is Valid`
          (bind _asbp_pawn_base (cast `/Game/RL/Core/BP_PawnBase` _attacktargetactor))
          (bind _output_get (set `local.TargetLocation` (`self.GetAimTargetPostion` _asbp_pawn_base)))
          (bind (_outhit _returnvalue) (`KismetSystemLibrary.LineTraceSingle` (+ (`self.K2_GetActorLocation` NewParam) (0.0 0.0 100.0)) _output_get "TraceTypeQuery4"))
          (if _returnvalue
            (return (== (`.HitActor` (`GameplayStatics.BreakHitResult` _outhit)) _attacktargetactor))
            (else
              (return false))))))))

(fn `OnStatChanged`
  (params (Stat :type "/Game/RL/Data/Enum/E_AIBehavior Enum" :default "NewEnumerator15"))
  (switch `/Game/RL/Data/Enum/E_AIBehavior` Stat
    (:`NewEnumerator15`
      (`self.SetMoveSpeed` (`self.InitSpeed`))
      (set `CharacterMovementComponent.bOrientRotationToMovement` false (`self.CharacterMovement`)))
    (:`NewEnumerator0`
      (`self.SetMoveSpeed` (`self.WalkSpeed`))
      (set `CharacterMovementComponent.bOrientRotationToMovement` true (`self.CharacterMovement`)))
    (:`NewEnumerator7`
      (set `CharacterMovementComponent.bOrientRotationToMovement` false (`self.CharacterMovement`)))
    (:`NewEnumerator16`
      (`self.SetMoveSpeed` (`self.JogSpeed`))
      (set `CharacterMovementComponent.bOrientRotationToMovement` true (`self.CharacterMovement`)))))

(fn `PlayAttackSound`
  (`GameplayStatics.SpawnSoundAtLocation` (`KismetArrayLibrary.Array_Random` (`self.Sound_Attack`)) (`self.K2_GetActorLocation`) (struct) 1.0 1.0 0.0 null null))

(fn `PlayDeadSound`
  (`GameplayStatics.SpawnSoundAtLocation` (`KismetArrayLibrary.Array_Random` (`self.Sound_Dead`)) (`self.K2_GetActorLocation`) (struct) 1.0 1.0 0.0 null null))

(fn `PlayHurtSound`
  (`GameplayStatics.SpawnSoundAtLocation` (`KismetArrayLibrary.Array_Random` (`self.Sound_Hurt`)) (`self.K2_GetActorLocation`) (struct) 1.0 1.0 0.0 null null))

(fn `PlayStartSound`
  (`GameplayStatics.SpawnSoundAtLocation` (`KismetArrayLibrary.Array_Random` (`self.Sound_Start`)) (`self.K2_GetActorLocation`) (struct) 1.0 1.0 0.0 null null))

(fn `SearchBestBlindage`
  (returns (Blindage :type "/Game/RL/SceneInstance/BP_AI_Blindage Object Reference"))
  (locals (TargetLocation :type "Vector Structure" :default (0.0 0.0 0.0)) (BlindageHeightAdjust :type "Float (double-precision)" :default 100.0) (BestWeight :type "Float (double-precision)" :default -1.0) (NearestBlindage :type "/Game/RL/SceneInstance/BP_AI_Blindage Object Reference") (LoopBody :type "/Game/RL/SceneInstance/BP_AI_Blindage Object Reference"))
  (bind _attacktargetactor (`self.GetAttackTargetActor`))
  (bind _attacktargetactor_2 (`self.GetAttackTargetActor`))
  (`/Engine/EditorBlueprintResources/StandardMacros.IsValid` _attacktargetactor
    (:`Is Valid`
      (bind _asbp_pawn_base (cast `/Game/RL/Core/BP_PawnBase` _attacktargetactor))
      (bind _output_get (set `local.TargetLocation` (`self.GetAimTargetPostion` _asbp_pawn_base)))
      (for _array_element (`self.Blindages`)
        (bind _output_get_2 (set `local.LoopBody` _array_element))
        (if (or (not (`/Game/RL/SceneInstance/BP_AI_Blindage.IsOccupied` _output_get_2)) (== (`/Game/RL/SceneInstance/BP_AI_Blindage.GetOccupant` _output_get_2) self))
          (bind (_outhit _returnvalue) (`KismetSystemLibrary.LineTraceSingle` (+ (`self.K2_GetActorLocation` _array_element) (`KismetMathLibrary.MakeVector` 0.0 0.0 (`local.BlindageHeightAdjust`))) _output_get "TraceTypeQuery4"))
          (if _returnvalue
            (bind (_bblockinghit _binitialoverlap _time _distance _location _impactpoint _normal _impactnormal _physmat _hitactor _hitcomponent _hitbonename _hititem _elementindex _faceindex _tracestart) (`GameplayStatics.BreakHitResult` _outhit))
            (if (== _hitactor _attacktargetactor)
              (if (<= (`self.GetAttackRange`) (`KismetMathLibrary.Vector_DistanceSquared` _tracestart (`self.K2_GetActorLocation` _attacktargetactor_2)))
                (cast `/Game/RL/Core/BP_PawnBase` _attacktargetactor_2)
                (if (> (`/Game/RL/SceneInstance/BP_AI_Blindage.GetWeight` (`local.LoopBody`) self) (`local.BestWeight`))
                  (set `local.BestWeight` 0.0)
                  (set `local.NearestBlindage` (`local.LoopBody`))))))))
      (return (`local.NearestBlindage`)))))

(fn `SetAI Stat`
  (params (AIStat :type "/Game/RL/Data/Enum/E_AIBehavior Enum" :default "NewEnumerator15"))
  (bind _output_get (set `self.AIStat` AIStat))
  (bind _asbp_monster_ai_controller (cast `/Game/RL/AI/BP_MonsterAI_Controller` (`AIBlueprintHelperLibrary.GetAIController` self)))
  (`/Game/RL/AI/BP_MonsterAI_Controller.SetAI Stat` _asbp_monster_ai_controller _output_get))

(fn `SetAttackTargetActor`
  (params (AttackTargetActor :type "Actor Object Reference"))
  (bind _asabp_monster (`self.GetMonsterAnimInstance`))
  (bind _output_get (set `self.AttackTargetActor` AttackTargetActor))
  (bind _asbp_pawn_base (cast `/Game/RL/Core/BP_PawnBase` _output_get)
    (:`then`
      (`/Game/RL/AI/Animation/ABP_Monster.SetAimTarget` _asabp_monster _asbp_pawn_base))
    (:`CastFailed`
      (`/Game/RL/AI/Animation/ABP_Monster.SetAimTarget` _asabp_monster null))))

(fn `SetMoveSpeed`
  (params (MaxWalkSpeed :type "Float (double-precision)"))
  (set `CharacterMovementComponent.MaxWalkSpeed` MaxWalkSpeed (`self.CharacterMovement`)))

(fn `UserConstructionScript`
  (`SceneComponent.SetVisibility` (`self.Widget`) (`self.bShowHealthUI`) false)
  (`SceneComponent.K2_AttachToComponent` (`self.WeaponChildActor`) (`self.Mesh`) (`self.Socket_Weapon`) "SnapToTarget" "SnapToTarget" "SnapToTarget" true))