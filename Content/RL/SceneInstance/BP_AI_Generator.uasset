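; Monster spawner actor that creates random-class monsters at generate points relative to itself, optionally on BeginPlay.
; Run fills either every point or a random count, tracking spawns in AliveMonsters and binding their death events.
; Deaths notify listeners; looping either replaces each casualty at a random point or reruns once all are dead.
; AutoAttackPlayer fakes player-instigated noise and damage perception events to aggro new spawns.
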(event `self.ReceiveBeginPlay`
  (if (`self.bAutoRun`)
    (`self.Run`)))

(event `Run`
  (bind _generatepoints (`self.GeneratePoints`))
  (if (`self.bRandom`)
    (bind _output_get (set `self.RadomNum` (`KismetMathLibrary.RandomIntegerInRange` (`self.RandomNumMin`) (`self.RandomNumMax`))))
    (for _index (range (`KismetMathLibrary.Clamp` _output_get 1 9))
      (if (> _index 0)
        (`self.SpawnMonster` (`|GetArrayItem` _generatepoints (mod _index (`KismetArrayLibrary.Array_LastIndex` _generatepoints))))
        (else
          (`self.SpawnMonster` (`|GetArrayItem` _generatepoints _index)))))
    (else
      (for _array_element (`self.GeneratePoints`)
        (`self.SpawnMonster` _array_element)))))

(event `OnMonsterDead`
  (params (DeathPawn :type "/Game/RL/Core/BP_PawnBase Object Reference") (SourceASC :type "FGComponent Object Reference") (Damage :type "Float (double-precision)") (`Hit result` :type "HitResult Structure"))
  (bind _returnvalue (`KismetArrayLibrary.Array_Length` (`self.AliveMonsters`)))
  (`KismetSystemLibrary.PrintString` (`KismetStringLibrary.Concat_StrStr` "Monster Dead:  " (`KismetSystemLibrary.GetDisplayName` DeathPawn)) false)
  (bind _asbp_monster_base (cast `/Game/RL/AI/BP_MonsterBase` DeathPawn))
  (clear `/Game/RL/Core/BP_PawnBase.OnDeath` _asbp_monster_base)
  (`KismetArrayLibrary.Array_RemoveItem` (`self.AliveMonsters`) _asbp_monster_base)
  (`self.OnAnyMonsterDead` _asbp_monster_base _returnvalue)
  (`KismetSystemLibrary.PrintString` (`KismetStringLibrary.Concat_StrStr` (`KismetSystemLibrary.GetDisplayName` self) "   MonsterDead  Left: = " (`KismetStringLibrary.Conv_IntToString` _returnvalue)) false)
  (if (`self.bLoopGenerate`)
    (if (`self.bGenerateEveryTimeWhenDead`)
      (`self.SpawnMonster` (`KismetArrayLibrary.Array_Random` (`self.GeneratePoints`)))
      (elif (== (`KismetArrayLibrary.Array_Length` (`self.AliveMonsters`)) 0)
        (`self.OnFinish`)
        (`self.Run`)))
    (elif (== (`KismetArrayLibrary.Array_Length` (`self.AliveMonsters`)) 0)
      (`self.OnFinish`))))

(fn `GetLeftMonster`
  (returns (ReturnValue :type Integer))
  (return (`KismetArrayLibrary.Array_Length` (`self.AliveMonsters`))))

(fn `SpawnMonster`
  (params (SpawnTransform :type "Transform Structure"))
  (bind _returnvalue (`GameplayStatics.GetPlayerPawn` 0))
  (bind _returnvalue_2 (`|SpawnActorFromClass` (`KismetArrayLibrary.Array_Random` (`self.MonsterClass`)) (`KismetMathLibrary.ComposeTransforms` SpawnTransform (`KismetMathLibrary.MakeTransform` (+ (.location (`self.GetTransform`)) (0.0 0.0 88.0)) (.rotation (`self.GetTransform`)) (.scale (`self.GetTransform`)))) "AdjustIfPossibleButAlwaysSpawn" "OverrideRootScale" self null))
  (`/Game/RL/AI/BP_MonsterBase.SetAI Stat` _returnvalue_2 (`self.DefaultStat`))
  (set `/Game/RL/AI/BP_MonsterBase.bShouldFindBindage` (`self.bShouldFindBindage`) _returnvalue_2)
  (`KismetArrayLibrary.Array_AddUnique` (`self.AliveMonsters`) _returnvalue_2)
  (add `/Game/RL/Core/BP_PawnBase.OnDeath` _returnvalue_2 (`|CreateDelegate` :!event `OnMonsterDead`))
  (`self.OnMonsterGenerate` _returnvalue_2)
  (`KismetSystemLibrary.PrintString` (`KismetStringLibrary.Concat_StrStr` "Monster Spawn" (`KismetSystemLibrary.GetDisplayName` _returnvalue_2)) false)
  (if (`self.bAutoAttackPlayer`)
    (bind _returnvalue_3 (`self.K2_GetActorLocation` _returnvalue_2))
    (`AISense_Hearing.ReportNoiseEvent` _returnvalue_3 1.0 _returnvalue 2000.0)
    (`AISense_Damage.ReportDamageEvent` _returnvalue_2 _returnvalue 1.0 _returnvalue_3 _returnvalue_3)))

(fn `UserConstructionScript`)