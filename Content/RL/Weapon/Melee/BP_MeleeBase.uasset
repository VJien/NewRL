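; BP_MeleeBase is a base melee weapon that reports hits on enemies to its owning pawn through the Gameplay Ability System.
; When AttackBox overlaps an enemy while CanAttack is set, a sphere trace toward the overlapped component produces a hit result.
; That result becomes target data in a melee WeaponHit gameplay event sent to the owner.
; A DoOnce gate blocks repeat hits until shortly after an overlap ends.
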(event `self.AttackBox.OnComponentBeginOverlap`
  (params (OverlappedComponent :type "PrimitiveComponent Object Reference") (OtherActor :type "Actor Object Reference") (OtherComp :type "PrimitiveComponent Object Reference") (OtherBodyIndex :type Integer) (bFromSweep :type Boolean) (SweepResult :type "HitResult Structure (by ref)"))
  (bind _ownerpawn (`self.OwnerPawn`))
  (bind _ownerpawn_2 (`self.OwnerPawn`))
  (if (!= OtherActor _ownerpawn_2)
    (if (`self.bCanAttack`)
      (if (`/Game/RL/FunctionLib/FLib_Utility.IsEnemy` OtherActor _ownerpawn_2)
        (`/Engine/EditorBlueprintResources/StandardMacros.DoOnce` false :!label _label
          (:`Completed`
            (bind _outhit (`KismetSystemLibrary.SphereTraceSingle` (`SceneComponent.K2_GetComponentLocation` (`self.AttackBox`)) (`SceneComponent.K2_GetComponentLocation` OtherComp) 10.0 "TraceTypeQuery4" false (`|MakeArray` (`self.OwnerPawn`) :!type "Actor Object Reference")))
            (`AbilitySystemBlueprintLibrary.SendGameplayEventToActor` _ownerpawn (struct :`TagName` "Event.Shared.WeaponHit.Melee") (make `GameplayEventData` (struct :`TagName` "Event.Shared.WeaponHit.Melee") _ownerpawn OtherActor null null (struct) (struct) (struct) 0.0 (`AbilitySystemBlueprintLibrary.AbilityTargetDataFromHitResult` _outhit)))))))))

(event `self.AttackBox.OnComponentEndOverlap`
  (params (OverlappedComponent :type "PrimitiveComponent Object Reference") (OtherActor :type "Actor Object Reference") (OtherComp :type "PrimitiveComponent Object Reference") (OtherBodyIndex :type Integer))
  (`KismetSystemLibrary.Delay` 0.2)
  (goto _label :!via `Reset`))

(fn `UserConstructionScript`
  (`parent.UserConstructionScript`))