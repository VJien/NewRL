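; Rocket projectile that plays a looping or launch audio cue on spawn and explodes with sound and particles at the impact point.
; If the actor it hits is an enemy of the instigator, it enables overlaps on a trace sphere and gathers the pawns inside.
; Each pawn with an ability system receives fixed physical damage through a set-by-caller gameplay effect, with no team check on the splash.
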(event `self.ReceiveBeginPlay`
  (`parent.ReceiveBeginPlay`)
  (`AudioComponent.Play` (`self.Sci-fi_Rocket_Projectile_01_Cue`) 0.0))

(fn `OnHit`
  (params (Hit :type "HitResult Structure (by ref)"))
  (locals (AllPanws :type "Array of Actor Object Reference"))
  (bind (_bblockinghit _binitialoverlap _time _distance _location _impactpoint _normal _impactnormal _physmat _hitactor) (`GameplayStatics.BreakHitResult` Hit))
  (`GameplayStatics.SpawnSoundAtLocation` (`self.HitSound`) _impactpoint (struct) 1.0 1.0 0.0 null null)
  (`GameplayStatics.SpawnEmitterAtLocation` "/Game/ThirdParty/Realistic_Starter_VFX_Pack_Vol2/Particles/Explosion/P_Explosion_Big_B.P_Explosion_Big_B" _impactpoint)
  (if (`/Game/RL/FunctionLib/FLib_Utility.IsEnemy` _hitactor (`self.GetInstigator`))
    (set `PrimitiveComponent.bGenerateOverlapEvents` true (`self.ExplodeTraceSphere`))
    (bind _output_get (set `local.AllPanws` (`PrimitiveComponent.GetOverlappingActors` (`self.ExplodeTraceSphere`) "/Game/RL/Core/BP_PawnBase.BP_PawnBase_C")))
    (for _array_element _output_get
      (`/Engine/EditorBlueprintResources/StandardMacros.IsValid` _array_element
        (:`Is Valid`
          (bind _returnvalue (`AbilitySystemBlueprintLibrary.GetAbilitySystemComponent` _array_element))
          (`/Engine/EditorBlueprintResources/StandardMacros.IsValid` _returnvalue
            (:`Is Valid`
              (`/Game/RL/FunctionLib/FLib_Utility.ApplyByCallerGameplayEffect` _returnvalue (struct :`TagName` "Attribute.Damage.Physics") "/FastGas/GE/ByCaller/GE_Override_Damage_Physics.GE_Override_Damage_Physics_C" 0.0 (struct) 50.0))))))))

(fn `UserConstructionScript`
  (`parent.UserConstructionScript`))