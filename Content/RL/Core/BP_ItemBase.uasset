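; BP_ItemBase is a base item Blueprint that declares a shared interaction surface for grabbing, dropping, using, highlighting and stowing items.
; Nearly every function is an overridable stub returning false or a default, including the grab pose, stat and hit and muzzle effect getters.
; Only TargetBeGrab has logic, storing the grabbing hand and returning true, while PuttoInventory and the construction script are empty.
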(event `/Game/RL/Interface/BPI_InteractableItem.PutToInventory`
  (params (Slot :type "/Game/RL/Data/Enum/E_EquipSlotType Enum" :default "NewEnumerator15") (TargetComp :type "SceneComponent Object Reference")))

(fn `CanGrab`
  (returns (result :type Boolean))
  (return false))

(fn `Drop`
  (params (Source :type "Actor Object Reference"))
  (returns (Success :type Boolean))
  (return false))

(fn `EnableHighLight`
  (params (bEnable :type Boolean))
  (returns (success :type Boolean))
  (return false))

(fn `GetGrabPose`
  (returns (Anim :type "AnimSequence Object Reference"))
  (return null))

(fn `GetHitEffects`
  (returns (Sound :type "SoundBase Object Reference") (FX :type "NiagaraSystem Object Reference"))
  (return null null))

(fn `GetMuzzleEffects`
  (returns (Sound :type "SoundBase Object Reference") (Niagara :type "NiagaraSystem Object Reference") (Particle :type "ParticleSystem Object Reference"))
  (return null null null))

(fn `GetStat`
  (returns (Stat :type "/Game/RL/Data/Enum/E_WeaponStat Enum"))
  (return "NewEnumerator0"))

(fn `TargetBeGrab`
  (params (SourcePawn :type "Pawn Object Reference") (Source :type "Actor Object Reference") (Hand :type "/Game/RL/Data/Enum/E_HandType Enum" :default "NewEnumerator7"))
  (returns (Success :type Boolean))
  (set `self.GrabedHand` Hand)
  (return true))

(fn `TryUseItem`
  (params (SoucreActor :type "Actor Object Reference") (SourcePawn :type "/Game/RL/Core/BP_PawnBase Object Reference"))
  (returns (success :type Boolean))
  (return false))

(fn `UserConstructionScript`)