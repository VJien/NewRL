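; BP_Start is a VR start trigger: a highlighted sphere the player grabs to fire the OnStart dispatcher.
; It binds to an overlapping BP_VR_Hand's grab event, clearing all bindings on that event when overlap ends.
; Grabbing disables collision, shows "GO !" and shrinks the sphere to zero with a timeline.
; It registers as ignored by the bullet time manager and turns the sphere toward the camera every tick.
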(event `self.ReceiveBeginPlay`
  (`/InteractionFramework/Components/Misc/BPC_HighLight.Init` (`self.BPC_HighLight`) (`|MakeArray` (`self.Sphere`) :!type "PrimitiveComponent Object Reference"))
  (`/Game/RL/Subsystem/BulletTimeManager/BP_BulletTimeManager.AddIgnoreActor` (subsystem `/Game/RL/Subsystem/BulletTimeManager/BP_BulletTimeManager`) self))

(event `self.ReceiveActorBeginOverlap`
  (params (OtherActor :type "Actor Object Reference"))
  (bind _asbp_vr_hand (cast `/Game/RL/Core/BP_VR_Hand` OtherActor))
  (add `/Game/RL/Core/BP_VR_Hand.OnGrabPressed` _asbp_vr_hand (delegate `OnGrab`)))

(event `OnGrab`
  (params (bGrab :type Boolean))
  (if bGrab
    (`PrimitiveComponent.SetCollisionEnabled` (`self.Sphere`) "NoCollision")
    (`self.OnStart`)
    (`TextRenderComponent.K2_SetText` (`self.TextRender`) "GO !")
    (bind (_direction _newtrack_0) (`Timeline|Start` :!via `PlayFromStart`)
      (:`Update`
        (`SceneComponent.SetWorldScale3D` (`self.Sphere`) (`KismetMathLibrary.Conv_DoubleToVector` (`KismetMathLibrary.Lerp` 0.5 0.0 _newtrack_0)))))))

(event `self.ReceiveActorEndOverlap`
  (params (OtherActor :type "Actor Object Reference"))
  (bind _asbp_vr_hand (cast `/Game/RL/Core/BP_VR_Hand` OtherActor))
  (clear `/Game/RL/Core/BP_VR_Hand.OnGrabPressed` _asbp_vr_hand))

(event `self.ReceiveTick`
  (params (DeltaSeconds :type "Float (single-precision)"))
  (`SceneComponent.K2_SetWorldRotation` (`self.Sphere`) (`KismetMathLibrary.FindLookAtRotation` (`self.K2_GetActorLocation`) (`self.K2_GetActorLocation` (`GameplayStatics.GetPlayerCameraManager` 0))) false false))

(fn `UserConstructionScript`)