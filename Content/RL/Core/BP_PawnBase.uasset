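; BP_PawnBase is a base pawn Blueprint providing shared camp, death and location-query logic.
; PostDeath calls the empty DoDeath function, then CallOnDeath with the pawn, source ASC, damage and hit result.
; CheckHealthIfDead calls DoDeath directly with zero damage when the pawn is not alive, skipping that notification.
; Helpers get and set the camp, return actor location as aim target, and derive foot location from the capsule.
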(event `self.ReceiveTick`
  (params (DeltaSeconds :type "Float (single-precision)")))

(event `Key|One`
  (params (Key :type "Key Structure")))

(event `/Game/RL/Interface/BPI_Camp.SetCamp`
  (params (Camp :type "/Game/RL/Data/Enum/E_Camp Enum" :default "NewEnumerator15"))
  (set `self.Camp` Camp))

(event `self.PostDeath`
  (params (SourceASC :type "FGComponent Object Reference") (Damage :type "Float (single-precision)") (HitResult :type "HitResult Structure"))
  (`self.DoDeath` SourceASC Damage HitResult)
  (`self.OnDeath` self SourceASC Damage HitResult))

(fn `CheckHealthIfDead`
  (if (not (`self.IsAlive`))
    (`self.DoDeath` null)))

(fn `DoDeath`
  (params (SourceASC :type "FGComponent Object Reference") (Damage :type "Float (double-precision)") (HitResult :type "HitResult Structure")))

(fn `GetAimTargetPostion`
  (returns (ReturnValue :type "Vector Structure"))
  (return (`self.K2_GetActorLocation`)))

(fn `GetCamp`
  (returns (Camp :type "/Game/RL/Data/Enum/E_Camp Enum"))
  (return (`self.Camp`)))

(fn `GetFootLocation`
  (returns (ReturnValue :type "Vector Structure"))
  (bind _capsulecomponent (`self.CapsuleComponent`))
  (return (- (`SceneComponent.K2_GetComponentLocation` _capsulecomponent) (`KismetMathLibrary.MakeVector` 0.0 0.0 (`CapsuleComponent.GetScaledCapsuleHalfHeight` _capsulecomponent)))))

(fn `UserConstructionScript`)