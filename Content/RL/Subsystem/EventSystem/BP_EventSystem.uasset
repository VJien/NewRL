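; BP_EventSystem is a message bus that routes UI messages to registered listeners by event ID.
; RegisterUIEvent asks a BPI_UIEvent object for its event IDs and adds it without duplicates to each listener array in the EventsCollection map.
; SendUIMessage calls OnMessageCallMessage on every listener of the message's EventID, pruning invalid ones during the loop.
; Init and tick events are empty, and there is no explicit unregister function.
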(event `self.OnInit`)

(event `self.OnTick`
  (params (DeltaTime :type "Float (single-precision)")))

(fn `RegisterUIEvent`
  (params (Target :type "Object Object Reference"))
  (locals (Objs :type "Array of Object Object Reference"))
  (bind _asbpi_uievent (cast `/Game/RL/Subsystem/EventSystem/UIEvent/BPI_UIEvent` Target))
  (bind _events (`/Game/RL/Subsystem/EventSystem/UIEvent/BPI_UIEvent.GetListenEvents` _asbpi_uievent))
  (for _array_element _events
    (bind (_value _returnvalue) (`BlueprintMapLibrary.Map_Find` (`self.EventsCollection`) _array_element))
    (if _returnvalue
      (bind _output_get (set `local.Objs` (`.Objs_5_A3B57B6B4F8668A41366FEA122E530C5` (break `/Game/RL/Subsystem/EventSystem/UIEvent/S_UIEventArray` _value))))
      (`KismetArrayLibrary.Array_AddUnique` _output_get Target)
      (`BlueprintMapLibrary.Map_Add` (`self.EventsCollection`) _array_element (make `/Game/RL/Subsystem/EventSystem/UIEvent/S_UIEventArray` (`local.Objs`)))
      (else
        (`BlueprintMapLibrary.Map_Add` (`self.EventsCollection`) _array_element (make `/Game/RL/Subsystem/EventSystem/UIEvent/S_UIEventArray` (`|MakeArray` Target)))))))

(fn `SendUIMessage`
  (params (UIMessage :type "/Game/RL/Subsystem/EventSystem/UIEvent/S_UIMessage Structure (by ref)"))
  (locals (Count :type Integer) (Objs :type "Array of Object Object Reference"))
  (bind _eventid (break `/Game/RL/Subsystem/EventSystem/UIEvent/S_UIMessage` UIMessage))
  (bind _objs (`local.Objs`))
  (bind _count (`local.Count`))
  (bind _objs_2 (`local.Objs`))
  (bind (_value _returnvalue) (`BlueprintMapLibrary.Map_Find` (`self.EventsCollection`) _eventid))
  (bind _output (`|GetArrayItem` _objs _count))
  (if _returnvalue
    (set `local.Objs` (`.Objs_5_A3B57B6B4F8668A41366FEA122E530C5` (break `/Game/RL/Subsystem/EventSystem/UIEvent/S_UIEventArray` _value)))
    (set `local.Count` 0)
    (if (< (`local.Count`) (`KismetArrayLibrary.Array_Length` _objs)) :!label _label
      (`/Engine/EditorBlueprintResources/StandardMacros.IsValid` _output
        (:`Is Valid`
          (message `/Game/RL/Subsystem/EventSystem/UIEvent/BPI_UIEvent.OnMessageCall` _output UIMessage)
          (`/Engine/EditorBlueprintResources/StandardMacros.IncrementInt` (`local.Count`)
            (:`  `
              (goto _label))))
        (:`Is Not Valid`
          (`KismetArrayLibrary.Array_Remove` _objs_2 _count)
          (setmembers `/Game/RL/Subsystem/EventSystem/UIEvent/S_UIEventArray` :`StructRef` _value :`Objs` _objs_2)
          (goto _label)))
      (else
        (`BlueprintMapLibrary.Map_Add` (`self.EventsCollection`) _eventid (make `/Game/RL/Subsystem/EventSystem/UIEvent/S_UIEventArray` (`local.Objs`)))))))