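; BP_Monster_Melee is a melee monster that attacks with a weapon held in a child actor, using the Gameplay Ability System.
; On BeginPlay it reads an attribute from the weapon and adds it to itself as attack through a runtime additive gameplay effect.
; DoAttack binds the finish callback, halts movement and activates GA_Melee.
; EnableWeaponAttack toggles the melee weapon's CanAttack flag.
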(event `self.ReceiveBeginPlay`
  (`parent.ReceiveBeginPlay`)
  ;[1 1 1] Add Attack From Weapon
  (bind _asbp_weapon_base (cast `/Game/RL/Weapon/BP_WeaponBase` (`ChildActorComponent.ChildActor` (`self.WeaponChildActor`))))
  (bind (_bsuccessfullyfoundattribute _returnvalue) (`AbilitySystemBlueprintLibrary.GetFloatAttributeBase` _asbp_weapon_base (struct :`AttributeName` "Attack_Final" :`Attribute` "/Script/FastGas.FGAttributeSetBase:Attack_Final")))
  (if _bsuccessfullyfoundattribute
    (`FGBlueprintLibrary.TryApplyGameplayEffectRumtime` (`self.AbilitySystemComponent`) (struct :`AttributeName` "Attack_BonusConstant" :`Attribute` "/Script/FastGas.FGAttributeSetBase:Attack_BonusConstant") _returnvalue "Additive")))

(event `self.ReceiveTick`
  (params (DeltaSeconds :type "Float (single-precision)"))
  (`parent.ReceiveTick` DeltaSeconds))

(fn `DoAttack`
  (params (Event :type "Delegate (by ref)"))
  (add `self.OnAttackFinish` Event)
  (`MovementComponent.StopMovementImmediately` (`self.CharacterMovement`))
  (`AbilitySystemComponent.TryActivateAbilityByClass` (`self.AbilitySystemComponent`) "/Game/RL/GAS/GA/GA_Melee.GA_Melee_C" true)
  (return))

(fn `EnableWeaponAttack`
  (params (bCanAttack :type Boolean))
  (bind _asbp_melee_base (cast `/Game/RL/Weapon/Melee/BP_MeleeBase` (`ChildActorComponent.ChildActor` (`self.WeaponChildActor`))))
  (set `/Game/RL/Weapon/Melee/BP_MeleeBase.bCanAttack` bCanAttack _asbp_melee_base))

(fn `UserConstructionScript`
  (`parent.UserConstructionScript`))