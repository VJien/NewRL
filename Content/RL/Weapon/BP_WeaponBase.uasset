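; Base VR weapon actor that handles grabbing, dropping, inventory holstering, firing and reloading through a weapon state enum and the Gameplay Ability System.
; Grabbing initializes GAS from the holder and restores saved ammo; drop and holstering save it again.
; Using it activates its first default ability, with helpers for bullets, effects and montages, while ammo changes use runtime gameplay effects.
; Tick updates a line-traced laser sight.
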(event `self.ReceiveBeginPlay`
  (`/InteractionFramework/Components/Misc/BPC_HighLight.Init` (`self.BPC_HighLight`) (`|MakeArray` (`self.Mesh`) :!type "PrimitiveComponent Object Reference"))
  (`self.InitSnapSource`)
  (`self.SetWeaponStat` "NewEnumerator0")
  (`KismetSystemLibrary.Delay` 0.2)
  (bind _asuw_bullet_num (cast `/Game/RL/Widget/UW_BulletNum` (`WidgetComponent.GetUserWidgetObject` (`self.BulletUI`))))
  (`/Game/RL/Widget/UW_BulletNum.InitBulletUI` _asuw_bullet_num (`self.AbilitySystemComponent`)))

(event `self.ReceiveTick`
  (params (DeltaSeconds :type "Float (single-precision)"))
  (`self.UpdateLazer`))

(event `PutToInventory_1`
  (params (Slot :type "/Game/RL/Data/Enum/E_EquipSlotType Enum" :default "NewEnumerator15") (TargetComp :type "SceneComponent Object Reference"))
  (set `self.DropTargetComp` TargetComp)
  (`self.K2_DetachFromActor` "KeepWorld" "KeepWorld" "KeepWorld")
  (`self.SetWeaponStat` "NewEnumerator10")
  (`TimelineComponent.PlayFromStart` (`self.ToInventory`))
  (set `self.bCanGrab` true)
  (`self.SaveLastBulletData`)
  (`self.Reset`))

(event `/Game/RL/Interface/BPI_InputReceiver.InputEvent_Trigger`
  (params (bPress :type Boolean) (Hand :type "/Game/RL/Data/Enum/E_HandType Enum" :default "NewEnumerator7")))

(event `self.Init`
  (params (InOwnerPawn :type "FGCharacter Object Reference"))
  (bind (_bsuccessfullyfoundattribute _returnvalue) (`AbilitySystemBlueprintLibrary.GetFloatAttribute` InOwnerPawn (struct :`AttributeName` "Attack_Final" :`Attribute` "/Script/FastGas.FGAttributeSetBase:Attack_Final")))
  (bind _abilitysystemcomponent (`self.AbilitySystemComponent`))
  ;[1 1 1] 初始化GAS
  (`parent.Init` InOwnerPawn)
  (if _bsuccessfullyfoundattribute
    (`/Engine/EditorBlueprintResources/StandardMacros.IsValid` _abilitysystemcomponent
      (:`Is Valid`
        (bind _returnvalue_2 (`AbilitySystemBlueprintLibrary.AssignTagSetByCallerMagnitude` (`AbilitySystemComponent.MakeOutgoingSpec` :`self` _abilitysystemcomponent :`GameplayEffectClass` "/FastGas/GE/ByCaller/GE_Add_Attack_Base.GE_Add_Attack_Base_C") (struct :`TagName` "Attribute.Attack.Base") _returnvalue))
        (`AbilitySystemComponent.BP_ApplyGameplayEffectSpecToSelf` (`self.AbilitySystemComponent`) _returnvalue_2)
        (`|ExecutionSequence`
          (:`then_0`
            (`/Engine/EditorBlueprintResources/StandardMacros.Gate` true :!label _label
              (:`Exit`
                (`self.SetCurrBullet` (`self.SavedBulletNum`))
                (`self.SetMaxBullet` (`self.SavedBulletNumMax`)))))
          (:`then_1`
            (goto _label :!via `Open`))))
      (:`Is Not Valid`
        (if true
          _)))))

(event `/Game/RL/Interface/BPI_InputReceiver.InputEvent_Grip`
  (params (bPress :type Boolean) (Hand :type "/Game/RL/Data/Enum/E_HandType Enum" :default "NewEnumerator7")))

(event `WaitReload`
  ;[1 1 1] Reload
  (`self.PlayReloadSound`)
  (`self.PlayReloadAnimation`)
  (`self.Reload Finish`))

(fn `AddCurrBullet`
  (params (Magnitude :type "Float (double-precision)"))
  (`FGBlueprintLibrary.TryApplyGameplayEffectRumtime` (`self.AbilitySystemComponent`) (struct :`AttributeName` "BulletNum_Default" :`Attribute` "/Script/FastGas.FGAttributeSetBase:BulletNum_Default") Magnitude "Additive"))

(fn `AddMaxBullet`
  (params (Magnitude :type "Float (double-precision)"))
  (`FGBlueprintLibrary.TryApplyGameplayEffectRumtime` (`self.AbilitySystemComponent`) (struct :`AttributeName` "BulletNum_Default_Max" :`Attribute` "/Script/FastGas.FGAttributeSetBase:BulletNum_Default_Max") Magnitude "Additive"))

(fn `CanGrab`
  (returns (result :type Boolean))
  (bind _weaponstat (`self.WeaponStat`))
  (return (and (`self.bCanGrab`) (or (`|EnumEquality` _weaponstat "NewEnumerator0") (`|EnumEquality` _weaponstat "NewEnumerator8")))))

(fn `Drop`
  (params (Source :type "Actor Object Reference"))
  (returns (Success :type Boolean))
  (`|ExecutionSequence`
    (:`then_0`
      (`self.SetWeaponStat` "NewEnumerator7")
      (`TimelineComponent.PlayFromStart` (`self.DropTimeline`))
      (`self.ResetWeapon`)
      (`self.SaveLastBulletData`)
      (`self.Reset`))
    (:`then_1`
      (return true))))

(fn `EnableHighLight`
  (params (bEnable :type Boolean))
  (returns (success :type Boolean))
  (`/InteractionFramework/Components/Misc/BPC_HighLight.EnableHighLight` (`self.BPC_HighLight`) bEnable)
  (return true))

(fn `Get Weapon Stat`
  (returns (WeaponStat :type "/Game/RL/Data/Enum/E_WeaponStat Enum"))
  (return (`self.WeaponStat`)))

(fn `GetGrabPose`
  (returns (Anim :type "AnimSequence Object Reference"))
  (return (`self.Anim_HandGrab`)))

(fn `GetHitEffects`
  (returns (Sound :type "SoundBase Object Reference") (FX :type "NiagaraSystem Object Reference"))
  (return null null))

(fn `GetMuzzleEffects`
  (returns (Sound :type "SoundBase Object Reference") (Niagara :type "NiagaraSystem Object Reference") (Particle :type "ParticleSystem Object Reference"))
  (return (`self.Sound_Shoot`) (`self.MuzllesSystem`) (`self.MuzlleParticle`)))

(fn `GetMuzzleTransform`
  (returns (ReturnValue :type "Transform Structure"))
  (return (`SceneComponent.GetSocketTransform` (`self.Mesh`) (`self.Socket_Mullze`) "RTS_World")))

(fn `GetStat`
  (returns (Stat :type "/Game/RL/Data/Enum/E_WeaponStat Enum"))
  (return (`self.WeaponStat`)))

(fn `GetWeaponBaseAnimInstance`
  (returns (`AsABP Weapon Base` :type "/Game/RL/Weapon/Anim/ABP_WeaponBase Object Reference"))
  (bind _asabp_weapon_base (cast `/Game/RL/Weapon/Anim/ABP_WeaponBase` (`SkeletalMeshComponent.GetAnimInstance` (`self.Mesh`))))
  (return _asabp_weapon_base))

(fn `GetWeaponFirePosition`
  (returns (ReturnValue :type "Transform Structure"))
  (return (`SceneComponent.GetSocketTransform` (`self.Mesh`) (`self.Socket_Shoot`) "RTS_World")))

(fn `InitSnapSource`)

(fn `PlayReloadAnimation`
  (bind _asabp_weapon_base (cast `/Game/RL/Weapon/Anim/ABP_WeaponBase` (`SkeletalMeshComponent.GetAnimInstance` (`self.Mesh`))))
  (`AnimInstance.Montage_Play` _asabp_weapon_base (`self.Anim_Reload`) 1.0 "MontageLength" 0.0 true))

(fn `PlayReloadSound`
  (`GameplayStatics.PlaySoundAtLocation` (`self.Sound_Reload`) (`self.K2_GetActorLocation`) (struct) 1.0 1.0 0.0 null null null))

(fn `PlayShootAnimation`
  (bind _asabp_weapon_base (cast `/Game/RL/Weapon/Anim/ABP_WeaponBase` (`SkeletalMeshComponent.GetAnimInstance` (`self.Mesh`))))
  (`AnimInstance.Montage_Play` _asabp_weapon_base (`self.Anim_Shoot`) 1.0 "MontageLength" 0.0 true))

(fn `Reload`
  (locals (Curr :type "Float (double-precision)" :default 0.0) (Max :type "Float (double-precision)" :default 0.0) (PerMag :type "Float (double-precision)" :default 0.0))
  (`self.WaitReload`)
  (`KismetSystemLibrary.PrintString` "准备换弹"))

(fn `Reload Finish`
  (locals (Curr :type "Float (double-precision)" :default 0.0) (Max :type "Float (double-precision)" :default 0.0) (PerMag :type "Float (double-precision)" :default 0.0))
  (`|ExecutionSequence`
    (:`then_0`
      (set `local.Curr` (`.ReturnValue` (`AbilitySystemBlueprintLibrary.GetFloatAttributeFromAbilitySystemComponent` (`self.AbilitySystemComponent`) (struct :`AttributeName` "BulletNum_Default" :`Attribute` "/Script/FastGas.FGAttributeSetBase:BulletNum_Default"))))
      (set `local.Max` (`.ReturnValue` (`AbilitySystemBlueprintLibrary.GetFloatAttributeFromAbilitySystemComponent` (`self.AbilitySystemComponent`) (struct :`AttributeName` "BulletNum_Default_Max" :`Attribute` "/Script/FastGas.FGAttributeSetBase:BulletNum_Default_Max"))))
      (set `local.PerMag` (`.ReturnValue` (`AbilitySystemBlueprintLibrary.GetFloatAttributeFromAbilitySystemComponent` (`self.AbilitySystemComponent`) (struct :`AttributeName` "BulletNum_Default_PerMag" :`Attribute` "/Script/FastGas.FGAttributeSetBase:BulletNum_Default_PerMag")))))
    (:`then_1`
      (if (<= (`local.Max`) 0.0)
        (return)
        (elif (>= (+ (`local.Max`) (`local.Curr`)) (`local.PerMag`))
          (`self.SetCurrBullet` (`local.PerMag`))
          (`self.AddMaxBullet` (- (`local.Curr`) (`local.PerMag`)))
          (else
            (`self.SetCurrBullet` (+ (`local.Max`) (`local.Curr`)))
            (`self.SetMaxBullet` 0.0)))))))

(fn `ReloadFromMag`
  (params (AdditiveBullet :type "Float (double-precision)"))
  (locals (Curr :type "Float (double-precision)" :default 0.0) (Max :type "Float (double-precision)" :default 0.0) (PerMag :type "Float (double-precision)" :default 0.0) (Add :type "Float (double-precision)"))
  (`|ExecutionSequence`
    (:`then_0`
      (set `local.Curr` (`.ReturnValue` (`AbilitySystemBlueprintLibrary.GetFloatAttributeFromAbilitySystemComponent` (`self.AbilitySystemComponent`) (struct :`AttributeName` "BulletNum_Default" :`Attribute` "/Script/FastGas.FGAttributeSetBase:BulletNum_Default"))))
      (set `local.Max` (`.ReturnValue` (`AbilitySystemBlueprintLibrary.GetFloatAttributeFromAbilitySystemComponent` (`self.AbilitySystemComponent`) (struct :`AttributeName` "BulletNum_Default_Max" :`Attribute` "/Script/FastGas.FGAttributeSetBase:BulletNum_Default_Max"))))
      (set `local.PerMag` (`.ReturnValue` (`AbilitySystemBlueprintLibrary.GetFloatAttributeFromAbilitySystemComponent` (`self.AbilitySystemComponent`) (struct :`AttributeName` "BulletNum_Default_PerMag" :`Attribute` "/Script/FastGas.FGAttributeSetBase:BulletNum_Default_PerMag"))))
      (set `local.Add` AdditiveBullet))
    (:`then_1`
      (if (< (+ (`local.Add`) (`local.Curr`)) (`local.PerMag`))
        (`self.AddCurrBullet` (`local.Add`))
        (else
          (`KismetSystemLibrary.PrintString` (`KismetStringLibrary.Concat_StrStr` "子弹 添加"))
          (`self.AddCurrBullet` (`local.PerMag`))
          (`self.AddMaxBullet` (- (+ (`local.Curr`) (`local.Add`)) (`local.PerMag`))))))))

(fn `ResetWeapon`
  (`self.K2_DetachFromActor` "KeepWorld" "KeepWorld" "KeepWorld")
  (`self.EnableHighLight` false)
  (set `self.bCanGrab` true)
  (`KismetArrayLibrary.Array_Clear` (`self.AttackIgnoreList`))
  (set `self.OwnerPawn` null))

(fn `SaveLastBulletData`
  (set `self.SavedBulletNum` (`.ReturnValue` (`AbilitySystemBlueprintLibrary.GetFloatAttributeFromAbilitySystemComponent` (`self.AbilitySystemComponent`) (struct :`AttributeName` "BulletNum_Default" :`Attribute` "/Script/FastGas.FGAttributeSetBase:BulletNum_Default"))))
  (set `self.SavedBulletNumMax` (`.ReturnValue` (`AbilitySystemBlueprintLibrary.GetFloatAttributeFromAbilitySystemComponent` (`self.AbilitySystemComponent`) (struct :`AttributeName` "BulletNum_Default_Max" :`Attribute` "/Script/FastGas.FGAttributeSetBase:BulletNum_Default_Max")))))

(fn `SetCurrBullet`
  (params (Magnitude :type "Float (double-precision)"))
  (`FGBlueprintLibrary.TryApplyGameplayEffectRumtime` (`self.AbilitySystemComponent`) (struct :`AttributeName` "BulletNum_Default" :`Attribute` "/Script/FastGas.FGAttributeSetBase:BulletNum_Default") Magnitude "Override"))

(fn `SetMaxBullet`
  (params (Magnitude :type "Float (double-precision)"))
  (`FGBlueprintLibrary.TryApplyGameplayEffectRumtime` (`self.AbilitySystemComponent`) (struct :`AttributeName` "BulletNum_Default_Max" :`Attribute` "/Script/FastGas.FGAttributeSetBase:BulletNum_Default_Max") Magnitude "Override"))

(fn `SetWeaponStat`
  (params (WeaponStat :type "/Game/RL/Data/Enum/E_WeaponStat Enum" :default "NewEnumerator0"))
  (set `self.WeaponStat` WeaponStat))

(fn `ShowLazer`
  (params (bShow :type Boolean))
  (set `self.bShowLazer` bShow))

(fn `SpawnBullet`
  (params (Transform :type "Transform Structure") (Container :type "FGGameplayEffectContainer Structure") (EventData :type "GameplayEventData Structure") (Level :type Integer))
  (bind _returnvalue (`|SpawnActorFromClass` (`self.BulletClass`) Transform "AlwaysSpawn" "OverrideRootScale" self (`self.AttackIgnoreList`) Container EventData Level (`self.OwnerPawn`)))
  (cast `/Game/RL/Core/BP_VR_Pawn` (`self.OwnerPawn`))
  (`/Game/RL/Subsystem/BulletTimeManager/BP_BulletTimeManager.AddIgnoreActor` (subsystem `/Game/RL/Subsystem/BulletTimeManager/BP_BulletTimeManager`) _returnvalue))

(fn `TargetBeGrab`
  (params (SourcePawn :type "Pawn Object Reference") (Source :type "Actor Object Reference") (Hand :type "/Game/RL/Data/Enum/E_HandType Enum" :default "NewEnumerator7"))
  (returns (Success :type Boolean))
  (locals (startTransform :type "Transform Structure") (VRPawn :type "/Game/RL/Core/BP_VR_Pawn Object Reference"))
  (`|ExecutionSequence`
    (:`then_0`
      (bind _asfgcharacter (cast `FGCharacter` SourcePawn))
      (`self.Init` _asfgcharacter))
    (:`then_1`
      (bind _asbp_vr_pawn (cast `/Game/RL/Core/BP_VR_Pawn` SourcePawn)
        (:`then`
          (`KismetArrayLibrary.Array_Append` (`self.AttackIgnoreList`) (`|MakeArray` _asbp_vr_pawn (`/Game/RL/Core/BP_VR_Pawn.LeftHand` _asbp_vr_pawn) (`/Game/RL/Core/BP_VR_Pawn.RightHand` _asbp_vr_pawn) self :!type "Actor Object Reference")))
        (:`CastFailed`
          (`KismetArrayLibrary.Array_Append` (`self.AttackIgnoreList`) (`|MakeArray` (`self.OwnerPawn`) self :!type "Actor Object Reference")))))
    (:`then_2`
      (if (`|EnumInequality` Hand "NewEnumerator7")
        (`self.EnableHighLight` false)
        (set `self.bCanGrab` false)
        (`self.SetWeaponStat` "NewEnumerator1")
        (return true)))))

(fn `TryAddBullet`
  (params (Num :type "Float (double-precision)"))
  (`KismetSystemLibrary.PrintString` "ADD ..................................." true true (struct :`R` 1.0 :`G` 0.998857 :`A` 1.0) 10.0)
  (bind _returnvalue (`AbilitySystemBlueprintLibrary.AssignTagSetByCallerMagnitude` (`AbilitySystemComponent.MakeOutgoingSpec` :`self` (`self.AbilitySystemComponent`) :`GameplayEffectClass` "/Game/RL/GAS/GE/ByCaller/Bullet/GE_Add_BulletNum_Base.GE_Add_BulletNum_Base_C") (struct :`TagName` "Attribute.BulletNum.1") Num))
  (`AbilitySystemComponent.BP_ApplyGameplayEffectSpecToSelf` (`self.AbilitySystemComponent`) _returnvalue))

(fn `TryUseItem`
  (params (SoucreActor :type "Actor Object Reference") (SourcePawn :type "/Game/RL/Core/BP_PawnBase Object Reference"))
  (returns (success :type Boolean))
  (bind _returnvalue (`AbilitySystemComponent.TryActivateAbilityByClass` (`self.AbilitySystemComponent`) (`|GetArrayItem` (`self.DefaultAbilities`)) true))
  (return _returnvalue))

(fn `UpdateLazer`
  (locals (NewLocalVar_0 :type "Array of Actor Object Reference") (LineScaleYZ :type "Float (double-precision)" :default 0.02) (PointScale :type "Float (double-precision)" :default 0.03))
  (bind _lazerline (`self.LazerLine`))
  (bind _linescaleyz (`local.LineScaleYZ`))
  (bind _linescaleyz_2 (`local.LineScaleYZ`))
  (bind _lazerpoint (`self.LazerPoint`))
  (bind _lazerpoint_2 (`self.LazerPoint`))
  (bind (_returnvalue_location _returnvalue_rotation) (`KismetMathLibrary.BreakTransform` (`SceneComponent.GetSocketTransform` (`self.Mesh`) (`self.Socket_Shoot`) "RTS_World")))
  (if (not (`|EnumEquality` (`/Game/RL/FunctionLib/FLib_Utility.GetVR Device`) "NewEnumerator1"))
    (set `self.bShowLazer` true))
  (`|ExecutionSequence`
    (:`then_0`
      (bind _asbp_vr_pawn (cast `/Game/RL/Core/BP_VR_Pawn` (`self.OwnerPawn`)))
      (set `local.NewLocalVar_0` (`/Game/RL/Core/BP_VR_Pawn.GetCommonIgnoreList` _asbp_vr_pawn)))
    (:`then_1`
      (`SceneComponent.SetVisibility` _lazerline (`self.bShowLazer`) false)
      (`SceneComponent.K2_SetWorldLocationAndRotation` _lazerline _returnvalue_location _returnvalue_rotation false false)
      (bind (_outhit _returnvalue) (`KismetSystemLibrary.LineTraceSingle` _returnvalue_location (+ _returnvalue_location (* (`KismetMathLibrary.GetForwardVector` _returnvalue_rotation) 9999.0)) "TraceTypeQuery4" false (`local.NewLocalVar_0`)))
      (if _returnvalue
        (bind (_bblockinghit _binitialoverlap _time _distance _location _impactpoint _normal _impactnormal _physmat _hitactor _hitcomponent _hitbonename _hititem _elementindex _faceindex _tracestart) (`GameplayStatics.BreakHitResult` _outhit))
        (`SceneComponent.SetWorldScale3D` (`self.LazerLine`) (`KismetMathLibrary.MakeVector` (/ (`KismetMathLibrary.VSize` (- _impactpoint _tracestart)) 100.0) _linescaleyz _linescaleyz))
        (`SceneComponent.K2_SetWorldLocation` _lazerpoint_2 _impactpoint false false)
        (`SceneComponent.SetVisibility` _lazerpoint_2 (`self.bShowLazer`) false)
        (`SceneComponent.SetWorldScale3D` _lazerpoint_2 (`KismetMathLibrary.Conv_DoubleToVector` (`local.PointScale`)))
        (else
          (`SceneComponent.SetWorldScale3D` (`self.LazerLine`) (`KismetMathLibrary.MakeVector` 100.0 _linescaleyz_2 _linescaleyz_2))
          (`SceneComponent.K2_SetWorldLocation` _lazerpoint (0.0 0.0 -5000.0) false false)
          (`SceneComponent.SetVisibility` _lazerpoint false false))))))

(fn `UserConstructionScript`
  (`parent.UserConstructionScript`)
  (`SceneComponent.K2_AttachToComponent` (`self.LazerPoint`) (`self.Mesh`) (`self.Socket_Lazer`) "SnapToTarget" "SnapToTarget" "SnapToTarget" true)
  (`SceneComponent.K2_AttachToComponent` (`self.LazerLine`) (`self.Mesh`) (`self.Socket_Lazer`) "SnapToTarget" "SnapToTarget" "SnapToTarget" true))